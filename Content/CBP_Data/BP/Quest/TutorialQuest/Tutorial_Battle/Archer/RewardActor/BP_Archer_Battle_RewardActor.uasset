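; Reward actor for the Archer battle tutorial that sets up an elevator and its remote control.
; On BeginPlay it spawns an animated floor object and copies in its end transform, rotation, play time and interaction settings.
; It then spawns a remote object, registers the floor as its target and labels both as the Archer elevator.
; Both spawned actors have BeginPlay called explicitly after configuration.
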(event `self.ReceiveBeginPlay`
  (bind _returnvalue (`|SpawnActorFromClass` "/Game/CBP_Data/BP/Object/Animation/BP_AnimationObject_Floor.BP_AnimationObject_Floor_C" (`self.Animation_Object_StartTransform`) "Undefined" "OverrideRootScale" null null))
  (bind _output_get (set `self.AnimationObject` _returnvalue))
  (set `CBP_NS_InteractionObject.widgetName` "아쳐 엘리베이터" _output_get)
  (set `CBP_AnimationObject.EndTransform` (`self.Animation_Object_EndTransform`) _output_get)
  (set `CBP_AnimationObject.ActorEndRotator` (`self.EndRotator`) _output_get)
  (set `CBP_NS_InteractionObject.isOnceInteraction` (`self.isOnceInteraction`) _output_get)
  (set `CBP_NS_InteractionObject.DirectInputType` (`self.isDirectInteraction`) _output_get)
  (set `CBP_AnimationObject.playTime` (`self.PlayTime`) _output_get)
  (bind _returnvalue_2 (`|SpawnActorFromClass` "/Game/CBP_Data/BP/Object/Animation/BP_RemoteObject.BP_RemoteObject_C" (`self.Remote_StartTransform`) "Undefined" "OverrideRootScale" null null))
  (bind _output_get_2 (set `self.Remote` _returnvalue_2))
  (set `CBP_NS_InteractionObject.widgetName` "아쳐 엘리베이터" _output_get_2)
  (`KismetArrayLibrary.Array_Add` (`CBP_RemoteObject.RemoteTargetActors` _output_get_2) (`self.AnimationObject`))
  (`CBP_AnimationObject.BeginPlay` (`self.AnimationObject`))
  (`CBP_RemoteObject.BeginPlay` (`self.Remote`)))

(fn `UserConstructionScript`)