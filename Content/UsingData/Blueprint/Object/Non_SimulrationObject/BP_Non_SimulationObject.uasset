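; BP_Non_SimulationObject is a prop actor that shows either a static or a skeletal mesh, with physics simulation turned off.
; Its construction script calls the parent's, then uses MeshType to destroy the unused mesh component and disable physics on the one that remains.
; SetScale and SetVisible switch on the same MeshType to set the active mesh's world scale or hidden-in-game state.
; The event graph holds only disabled placeholder events.
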(fn `Set Scale`
  (params (Scale :type "Vector Structure"))
  (switch `/Game/UsingData/Blueprint/Enum/Object/E_MeshType` (`self.Mesh Type`)
    (:`NewEnumerator1`
      (`SceneComponent.SetWorldScale3D` (`self.StaticMesh`) (`local.Scale`)))
    (:`NewEnumerator2`
      (`SceneComponent.SetWorldScale3D` (`self.SkeletalMesh`) (`local.Scale`)))))

(fn `Set Visible`
  (params (`New Hidden` :type Boolean))
  (switch `/Game/UsingData/Blueprint/Enum/Object/E_MeshType` (`self.Mesh Type`)
    (:`NewEnumerator1`
      (`SceneComponent.SetHiddenInGame` (`self.StaticMesh`) (`local.New Hidden`) false))
    (:`NewEnumerator2`
      (`SceneComponent.SetHiddenInGame` (`self.SkeletalMesh`) (`local.New Hidden`) false))))

(fn `UserConstructionScript`
  (`parent.UserConstructionScript`)
  (switch `/Game/UsingData/Blueprint/Enum/Object/E_MeshType` (`self.Mesh Type`)
    (:`NewEnumerator1`
      (`ActorComponent.K2_DestroyComponent` (`self.SkeletalMesh`))
      (`PrimitiveComponent.SetSimulatePhysics` (`self.StaticMesh`) false))
    (:`NewEnumerator2`
      (`ActorComponent.K2_DestroyComponent` (`self.StaticMesh`))
      (`PrimitiveComponent.SetSimulatePhysics` (`self.SkeletalMesh`) false))))