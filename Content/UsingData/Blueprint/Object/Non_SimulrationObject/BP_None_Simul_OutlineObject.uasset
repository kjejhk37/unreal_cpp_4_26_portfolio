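; Non-simulation object actor that carries a duplicate outline mesh for showing an outline around its static or skeletal mesh.
; The construction script switches on MeshType, destroys the unused outline component, then copies the source mesh onto the other, applies an outline material and attaches it to the source.
; SetHiddenOutline toggles the in-game visibility of whichever outline component matches the type.
; The event graph holds only disabled default events.
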(fn `Set Hidden Outline`
  (params (Hidden :type Boolean))
  (switch `/Game/UsingData/Blueprint/Enum/Object/E_MeshType` (`self.Mesh Type`)
    (:`NewEnumerator1`
      (`SceneComponent.SetHiddenInGame` (`self.Outline_StaticMesh`) (`local.Hidden`) false))
    (:`NewEnumerator2`
      (`SceneComponent.SetHiddenInGame` (`self.Outline_SkeletalMesh`) (`local.Hidden`) false))))

(fn `UserConstructionScript`
  (bind _outline_staticmesh (`self.Outline_StaticMesh`))
  (bind _outline_skeletalmesh (`self.Outline_SkeletalMesh`))
  (`parent.UserConstructionScript`)
  (switch `/Game/UsingData/Blueprint/Enum/Object/E_MeshType` (`self.Mesh Type`)
    (:`NewEnumerator1`
      (`ActorComponent.K2_DestroyComponent` (`self.Outline_SkeletalMesh`))
      (`StaticMeshComponent.SetStaticMesh` _outline_staticmesh (`StaticMeshComponent.StaticMesh` (`self.StaticMesh`)))
      (`PrimitiveComponent.SetMaterial` _outline_staticmesh 0 "/Game/UsingData/Material/Outline/BPM_OutlineMaterail.BPM_OutlineMaterail")
      (`SceneComponent.K2_AttachToComponent` (`self.Outline_StaticMesh`) (`self.StaticMesh`) "None" "KeepRelative" "KeepRelative" "KeepRelative" true))
    (:`NewEnumerator2`
      (`ActorComponent.K2_DestroyComponent` (`self.Outline_StaticMesh`))
      (`SkinnedMeshComponent.SetSkinnedAssetAndUpdate` _outline_skeletalmesh (`SkinnedMeshComponent.SkeletalMesh` (`self.SkeletalMesh`)) true)
      (`PrimitiveComponent.SetMaterial` _outline_skeletalmesh 0 "/Game/UsingData/Material/Outline/BPM_OutlineMaterail.BPM_OutlineMaterail")
      (`SceneComponent.K2_AttachToComponent` (`self.Outline_SkeletalMesh`) (`self.SkeletalMesh`) "None" "KeepRelative" "KeepRelative" "KeepRelative" true))))