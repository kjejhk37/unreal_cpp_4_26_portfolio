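; BP_AnimationObject is an interactable, key-locked object that plays an open or close timeline.
; On BeginPlay it registers itself with every key in its Keys array.
; UsingKey removes a matching key and sets CanOpen once none remain.
; A successful parent Interaction plays the OpenOrClose timeline forward when CanOpen is true, otherwise reverses it.
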(event `self.ReceiveBeginPlay`
  (`parent.ReceiveBeginPlay`)
  (for _array_element (`self.Keys`)
    (`/Game/UsingData/Blueprint/Object/SimulationObject/InteractionObject/MoveObject/KeyObject/BP_KeyObject.Resister Animation Object` _array_element self)))

(event `Open`
  (`Timeline|Open Or Close` :!label _label))

(event `Close`
  (goto _label :!via `Reverse`))

(fn `Interaction`
  (params (`Interaction Actor` :type "Actor Object Reference"))
  (returns (`Interaction Success` :type Boolean) (`Result Actor` :type "Actor Object Reference"))
  (bind _interaction_success (`parent.Interaction` `Interaction Actor`))
  (if _interaction_success
    (if (`self.Can Open`)
      (`self. Open`)
      (else
        (`self.Close`)))
    (return true null)))

(fn `UserConstructionScript`
  (`parent.UserConstructionScript`))

(fn `Using Key`
  (params (Key :type "/Game/UsingData/Blueprint/Object/SimulationObject/InteractionObject/MoveObject/KeyObject/BP_KeyObject Object Reference"))
  (returns (Success :type Boolean))
  (if (`KismetArrayLibrary.Array_Contains` (`self.Keys`) Key)
    (`KismetArrayLibrary.Array_RemoveItem` (`self.Keys`) Key)
    (set `self.Can Open` (<= (`KismetArrayLibrary.Array_Length` (`self.Keys`)) 0))
    (return true)
    (else
      (return false))))