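; Non-simulation interaction object actor that offers a configurable mesh type and interaction collision shape.
; The construction script attaches the selected box, sphere or capsule component to the chosen static or skeletal mesh, then destroys the two unused shapes.
; Its Interaction function is a stub that always reports success and returns the actor passed to it, and the event graph holds only disabled default events.
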(fn `Interaction`
  (params (`Interaction Actor` :type "Actor Object Reference"))
  (returns (`Interaction Success` :type Boolean) (`Result Actor` :type "Actor Object Reference"))
  (return true `Interaction Actor`))

(fn `UserConstructionScript`
  (bind _interaction_type (`self.Interaction Type`))
  (`parent.UserConstructionScript`)
  (`|ExecutionSequence`
    (:`then_0`
      (switch `/Game/UsingData/Blueprint/Enum/Object/E_MeshType` (`self.Mesh Type`)
        (:`NewEnumerator1`
          (switch `/Game/UsingData/Blueprint/Enum/Object/E_CollsionType` _interaction_type
            (:`NewEnumerator1`
              (`SceneComponent.K2_AttachToComponent` (`self.Interaction Box`) (`self.StaticMesh`) "None" "KeepRelative" "KeepRelative" "KeepRelative" true))
            (:`NewEnumerator2`
              (`SceneComponent.K2_AttachToComponent` (`self.Interaction Sphere`) (`self.StaticMesh`) "None" "KeepRelative" "KeepRelative" "KeepRelative" true))
            (:`NewEnumerator3`
              (`SceneComponent.K2_AttachToComponent` (`self.Interaction Capsule`) (`self.StaticMesh`) "None" "KeepRelative" "KeepRelative" "KeepRelative" true))))
        (:`NewEnumerator2`
          (switch `/Game/UsingData/Blueprint/Enum/Object/E_CollsionType` _interaction_type
            (:`NewEnumerator1`
              (`SceneComponent.K2_AttachToComponent` (`self.Interaction Box`) (`self.SkeletalMesh`) "None" "KeepRelative" "KeepRelative" "KeepRelative" true))
            (:`NewEnumerator2`
              (`SceneComponent.K2_AttachToComponent` (`self.Interaction Sphere`) (`self.SkeletalMesh`) "None" "KeepRelative" "KeepRelative" "KeepRelative" true))
            (:`NewEnumerator3`
              (`SceneComponent.K2_AttachToComponent` (`self.Interaction Capsule`) (`self.SkeletalMesh`) "None" "KeepRelative" "KeepRelative" "KeepRelative" true))))))
    (:`then_1`
      (switch `/Game/UsingData/Blueprint/Enum/Object/E_CollsionType` (`self.Interaction Type`)
        (:`NewEnumerator1`
          (`ActorComponent.K2_DestroyComponent` (`self.Interaction Sphere`))
          (`ActorComponent.K2_DestroyComponent` (`self.Interaction Capsule`)))
        (:`NewEnumerator2`
          (`ActorComponent.K2_DestroyComponent` (`self.Interaction Box`))
          (`ActorComponent.K2_DestroyComponent` (`self.Interaction Capsule`)))
        (:`NewEnumerator3`
          (`ActorComponent.K2_DestroyComponent` (`self.Interaction Box`))
          (`ActorComponent.K2_DestroyComponent` (`self.Interaction Sphere`)))))))