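; BP_PairWeapon is the companion piece of a paired weapon, following a main weapon through pickup, equip and drop.
; Pickup makes the character its Instigator, attaches it unequipped, hides the outline and rescales; SetEquip delegates attachment to the character and toggles visibility.
; Dropping reattaches the static or skeletal mesh to the main weapon's PairWeaponSocket and clears the Instigator.
; GetDamage exposes Damage, while Activate and Deactivate are stubs returning false.
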(fn `Activate`
  (params (success :type Boolean))
  (returns (Succsses :type Boolean))
  (return false))

(fn `Deactivate`
  (params (success :type Boolean))
  (returns (Succses :type Boolean))
  (return false))

(fn `Dropping Pair Weapon`
  (params (`Main Weapon` :type "Actor Object Reference"))
  (returns (Success :type Boolean))
  (bind _asbp_weapon_object (cast `/Game/UsingData/Blueprint/Object/SimulationObject/InteractionObject/MainWeaponObject/BP_WeaponObject` `Main Weapon`)
    (:`then`
      (switch `/Game/UsingData/Blueprint/Enum/Object/E_MeshType` (`self.Mesh Type`)
        (:`NewEnumerator1`
          (`SceneComponent.K2_AttachToComponent` (`self.StaticMesh`) (`/Game/UsingData/Blueprint/Object/SimulationObject/InteractionObject/MainWeaponObject/BP_WeaponObject.PairWeapon Socket` _asbp_weapon_object) "None" "KeepRelative" "KeepRelative" "KeepRelative" true))
        (:`NewEnumerator2`
          (`SceneComponent.K2_AttachToComponent` (`self.SkeletalMesh`) (`/Game/UsingData/Blueprint/Object/SimulationObject/InteractionObject/MainWeaponObject/BP_WeaponObject.PairWeapon Socket` _asbp_weapon_object) "None" "KeepRelative" "KeepRelative" "KeepRelative" true)))
      (set `self.Instigator` null)
      (`self.Set Scale` (`self.Pair Weapon Scale`))
      (return true))
    (:`CastFailed`
      (return false))))

(fn `Get Damage`
  (returns (Damage :type "Float (double-precision)"))
  (return (`self.Damage`)))

(fn `Pick Up Pair Weapon`
  (params (Actor :type "Actor Object Reference"))
  (returns (Success :type Boolean))
  (bind _asbp_character (cast `/Game/UsingData/Blueprint/Character/BP_Character` Actor)
    (:`then`
      (set `self.Instigator` _asbp_character)
      (`self.Set Equip` false)
      (`self.Set Hidden Outline` true)
      (`self.Set Scale` (`self.Pair Weapon Scale`))
      (return true))
    (:`CastFailed`
      (return false))))

(fn `Set Equip`
  (params (Equip :type Boolean))
  (bind _equip (`local.Equip`))
  (bind _asbp_character (cast `/Game/UsingData/Blueprint/Character/BP_Character` (`self.GetInstigator`)))
  (`/Game/UsingData/Blueprint/Character/BP_Character.Attach Actor To Character` _asbp_character self _equip)
  (`self.Set Visible` (not _equip)))

(fn `UserConstructionScript`
  (`parent.UserConstructionScript`))