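; Base Blueprint for a paired melee weapon that shows a particle trail while the weapon is active.
; The construction script attaches the particle component to the static or skeletal mesh according to MeshType, or destroys it when the type is None.
; Activate and Deactivate extend the parent behavior by beginning and ending trails between the Trail_Start and Trail_End sockets.
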(event `self.Particle_Activate`
  (`ParticleSystemComponent.BeginTrails` (`self.ParticleSystem`) "Trail_Start" "Trail_End" "ETrailWidthMode_FromCentre" 1.0))

(event `self.Particle_DeActivate`
  (`ParticleSystemComponent.EndTrails` (`self.ParticleSystem`)))

(fn `Activate`
  (params (success :type Boolean))
  (returns (Succsses :type Boolean))
  (bind _succsses (`parent.Activate` success))
  (`self.Particle_Activate`)
  (return _succsses))

(fn `Deactivate`
  (params (success :type Boolean))
  (returns (Succses :type Boolean))
  (bind _succses (`parent.Deactivate` success))
  (`self.Particle_DeActivate`)
  (return _succses))

(fn `UserConstructionScript`
  (`parent.UserConstructionScript`)
  (switch `/Game/UsingData/Blueprint/Enum/Object/E_MeshType` (`self.Mesh Type`)
    (:`NewEnumerator0`
      (`ActorComponent.K2_DestroyComponent` (`self.ParticleSystem`)))
    (:`NewEnumerator1`
      (`SceneComponent.K2_AttachToComponent` (`self.ParticleSystem`) (`self.StaticMesh`) "None" "KeepRelative" "KeepRelative" "KeepRelative" true))
    (:`NewEnumerator2`
      (`SceneComponent.K2_AttachToComponent` (`self.ParticleSystem`) (`self.SkeletalMesh`) "None" "KeepRelative" "KeepRelative" "KeepRelative" true))))