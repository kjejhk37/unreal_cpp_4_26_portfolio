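; Configurable physics object that pairs an optional static or skeletal mesh with an optional box, sphere or capsule simulation body.
; The construction script destroys unused components, attaches the mesh to the chosen shape and simulates that shape with mesh collision off, or the mesh itself without one.
; Scale, simulation and impulse functions target that active body, while visibility and mesh-scale functions target the mesh.
; Set Position and Set Rotation are empty.
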(fn `Set Impulse`
  (params (`Is At Location?` :type Boolean) (Power :type "Float (double-precision)") (Velocity :type "Vector Structure") (Location :type "Vector Structure"))
  (locals (Impulse :type "Vector Structure"))
  (set `local.Impulse` (* Velocity Power))
  (if `Is At Location?`
    (switch `/Game/UsingData/Blueprint/Enum/Object/E_SimulationType` (`self.Simulation Type`)
      (:`NewEnumerator0`
        (switch `/Game/UsingData/Blueprint/Enum/Object/E_MeshType` (`self.MeshType`)
          (:`NewEnumerator1`
            (`PrimitiveComponent.AddImpulseAtLocation` (`self.StaticMesh`) (`local.Impulse`) (`local.Location`) "None"))
          (:`NewEnumerator2`
            (`PrimitiveComponent.AddImpulseAtLocation` (`self.SkeletalMesh`) (`local.Impulse`) (`local.Location`) "None"))))
      (:`NewEnumerator4`
        (`PrimitiveComponent.AddImpulseAtLocation` (`self.Simulation Box`) (`local.Impulse`) (`local.Location`) "None"))
      (:`NewEnumerator5`
        (`PrimitiveComponent.AddImpulseAtLocation` (`self.Simulation Sphere`) (`local.Impulse`) (`local.Location`) "None"))
      (:`NewEnumerator6`
        (`PrimitiveComponent.AddImpulseAtLocation` (`self.Simulation Capsule`) (`local.Impulse`) (`local.Location`) "None")))
    (else
      (switch `/Game/UsingData/Blueprint/Enum/Object/E_SimulationType` (`self.Simulation Type`)
        (:`NewEnumerator0`
          (switch `/Game/UsingData/Blueprint/Enum/Object/E_MeshType` (`self.MeshType`)
            (:`NewEnumerator1`
              (`PrimitiveComponent.AddImpulse` (`self.StaticMesh`) (`local.Impulse`) "None" true))
            (:`NewEnumerator2`
              (`PrimitiveComponent.AddImpulse` (`self.SkeletalMesh`) (`local.Impulse`) "None" true))))
        (:`NewEnumerator4`
          (`PrimitiveComponent.AddImpulse` (`self.Simulation Box`) (`local.Impulse`) "None" true))
        (:`NewEnumerator5`
          (`PrimitiveComponent.AddImpulse` (`self.Simulation Sphere`) (`local.Impulse`) "None" true))
        (:`NewEnumerator6`
          (`PrimitiveComponent.AddImpulse` (`self.Simulation Capsule`) (`local.Impulse`) "None" true))))))

(fn `Set Position`
  (params (Position :type "Vector Structure")))

(fn `Set Rotation`
  (params (Rotation :type "Vector Structure")))

(fn `Set Scale`
  (params (Scale :type "Vector Structure"))
  (switch `/Game/UsingData/Blueprint/Enum/Object/E_SimulationType` (`self.Simulation Type`)
    (:`NewEnumerator0`
      (switch `/Game/UsingData/Blueprint/Enum/Object/E_MeshType` (`self.MeshType`)
        (:`NewEnumerator1`
          (`SceneComponent.SetWorldScale3D` (`self.StaticMesh`) (`local.Scale`)))
        (:`NewEnumerator2`
          (`SceneComponent.SetWorldScale3D` (`self.SkeletalMesh`) (`local.Scale`)))))
    (:`NewEnumerator4`
      (`SceneComponent.SetWorldScale3D` (`self.Simulation Box`) (`local.Scale`)))
    (:`NewEnumerator5`
      (`SceneComponent.SetWorldScale3D` (`self.Simulation Sphere`) (`local.Scale`)))
    (:`NewEnumerator6`
      (`SceneComponent.SetWorldScale3D` (`self.Simulation Capsule`) (`local.Scale`)))))

(fn `Set Scale Mesh`
  (params (Scale :type "Vector Structure"))
  (switch `/Game/UsingData/Blueprint/Enum/Object/E_MeshType` (`self.MeshType`)
    (:`NewEnumerator1`
      (`SceneComponent.SetWorldScale3D` (`self.StaticMesh`) (`local.Scale`)))
    (:`NewEnumerator2`
      (`SceneComponent.SetWorldScale3D` (`self.SkeletalMesh`) (`local.Scale`)))))

(fn `Set Simulation`
  (params (Enable :type Boolean))
  (switch `/Game/UsingData/Blueprint/Enum/Object/E_SimulationType` (`self.Simulation Type`)
    (:`NewEnumerator0`
      (switch `/Game/UsingData/Blueprint/Enum/Object/E_MeshType` (`self.MeshType`)
        (:`NewEnumerator1`
          (`PrimitiveComponent.SetSimulatePhysics` (`self.StaticMesh`) (`local.Enable`)))
        (:`NewEnumerator2`
          (`PrimitiveComponent.SetSimulatePhysics` (`self.SkeletalMesh`) (`local.Enable`)))))
    (:`NewEnumerator4`
      (`PrimitiveComponent.SetSimulatePhysics` (`self.Simulation Box`) (`local.Enable`)))
    (:`NewEnumerator5`
      (`PrimitiveComponent.SetSimulatePhysics` (`self.Simulation Sphere`) (`local.Enable`)))
    (:`NewEnumerator6`
      (`PrimitiveComponent.SetSimulatePhysics` (`self.Simulation Capsule`) (`local.Enable`)))))

(fn `Set Visible`
  (params (`New Hidden` :type Boolean))
  (switch `/Game/UsingData/Blueprint/Enum/Object/E_MeshType` (`self.MeshType`)
    (:`NewEnumerator1`
      (`SceneComponent.SetHiddenInGame` (`self.StaticMesh`) (`local.New Hidden`) false))
    (:`NewEnumerator2`
      (`SceneComponent.SetHiddenInGame` (`self.SkeletalMesh`) (`local.New Hidden`) false))))

(fn `UserConstructionScript`
  (bind _staticmesh (`self.StaticMesh`))
  (bind _meshtype (`self.MeshType`))
  (bind _skeletalmesh (`self.SkeletalMesh`))
  (`|ExecutionSequence`
    (:`then_0`
      (switch `/Game/UsingData/Blueprint/Enum/Object/E_MeshType` (`self.MeshType`)
        (:`NewEnumerator0`
          (`ActorComponent.K2_DestroyComponent` (`self.StaticMesh`))
          (`ActorComponent.K2_DestroyComponent` (`self.SkeletalMesh`)))
        (:`NewEnumerator1`
          (`ActorComponent.K2_DestroyComponent` (`self.SkeletalMesh`)))
        (:`NewEnumerator2`
          (`ActorComponent.K2_DestroyComponent` (`self.StaticMesh`)))))
    (:`then_1`
      (switch `/Game/UsingData/Blueprint/Enum/Object/E_SimulationType` (`self.Simulation Type`)
        (:`NewEnumerator0`
          (`ActorComponent.K2_DestroyComponent` (`self.Simulation Box`))
          (`ActorComponent.K2_DestroyComponent` (`self.Simulation Sphere`))
          (`ActorComponent.K2_DestroyComponent` (`self.Simulation Capsule`)))
        (:`NewEnumerator4`
          (`ActorComponent.K2_DestroyComponent` (`self.Simulation Sphere`))
          (`ActorComponent.K2_DestroyComponent` (`self.Simulation Capsule`)))
        (:`NewEnumerator5`
          (`ActorComponent.K2_DestroyComponent` (`self.Simulation Box`))
          (`ActorComponent.K2_DestroyComponent` (`self.Simulation Capsule`)))
        (:`NewEnumerator6`
          (`ActorComponent.K2_DestroyComponent` (`self.Simulation Box`))
          (`ActorComponent.K2_DestroyComponent` (`self.Simulation Sphere`)))))
    (:`then_2`
      (switch `/Game/UsingData/Blueprint/Enum/Object/E_SimulationType` (`self.Simulation Type`)
        (:`NewEnumerator0`
          (switch `/Game/UsingData/Blueprint/Enum/Object/E_MeshType` _meshtype))
        (:`NewEnumerator4`
          (switch `/Game/UsingData/Blueprint/Enum/Object/E_MeshType` _meshtype
            (:`NewEnumerator1`
              (`SceneComponent.K2_AttachToComponent` (`self.StaticMesh`) (`self.Simulation Box`) "None" "KeepRelative" "KeepRelative" "KeepRelative" true))
            (:`NewEnumerator2`
              (`SceneComponent.K2_AttachToComponent` (`self.SkeletalMesh`) (`self.Simulation Box`) "None" "KeepRelative" "KeepRelative" "KeepRelative" true))))
        (:`NewEnumerator5`
          (switch `/Game/UsingData/Blueprint/Enum/Object/E_MeshType` _meshtype
            (:`NewEnumerator1`
              (`SceneComponent.K2_AttachToComponent` (`self.StaticMesh`) (`self.Simulation Sphere`) "None" "KeepRelative" "KeepRelative" "KeepRelative" true))
            (:`NewEnumerator2`
              (`SceneComponent.K2_AttachToComponent` (`self.SkeletalMesh`) (`self.Simulation Sphere`) "None" "KeepRelative" "KeepRelative" "KeepRelative" true))))
        (:`NewEnumerator6`
          (switch `/Game/UsingData/Blueprint/Enum/Object/E_MeshType` _meshtype
            (:`NewEnumerator1`
              (`SceneComponent.K2_AttachToComponent` (`self.StaticMesh`) (`self.Simulation Capsule`) "None" "KeepRelative" "KeepRelative" "KeepRelative" true))
            (:`NewEnumerator2`
              (`SceneComponent.K2_AttachToComponent` (`self.SkeletalMesh`) (`self.Simulation Capsule`) "None" "KeepRelative" "KeepRelative" "KeepRelative" true))))))
    (:`then_3`
      (switch `/Game/UsingData/Blueprint/Enum/Object/E_SimulationType` (`self.Simulation Type`)
        (:`NewEnumerator0`
          (switch `/Game/UsingData/Blueprint/Enum/Object/E_MeshType` (`self.MeshType`)
            (:`NewEnumerator1`
              (`PrimitiveComponent.SetSimulatePhysics` (`self.StaticMesh`) true))
            (:`NewEnumerator2`
              (`PrimitiveComponent.SetSimulatePhysics` (`self.SkeletalMesh`) true))))
        (:`NewEnumerator4`
          (`PrimitiveComponent.SetSimulatePhysics` (`self.Simulation Box`) true)
          (switch `/Game/UsingData/Blueprint/Enum/Object/E_MeshType` (`self.MeshType`) :!label _label
            (:`NewEnumerator1`
              (`PrimitiveComponent.SetSimulatePhysics` _staticmesh false)
              (`PrimitiveComponent.SetCollisionEnabled` _staticmesh "NoCollision"))
            (:`NewEnumerator2`
              (`PrimitiveComponent.SetSimulatePhysics` _skeletalmesh false)
              (`PrimitiveComponent.SetCollisionEnabled` _skeletalmesh "NoCollision"))))
        (:`NewEnumerator5`
          (`PrimitiveComponent.SetSimulatePhysics` (`self.Simulation Sphere`) true)
          (goto _label))
        (:`NewEnumerator6`
          (`PrimitiveComponent.SetSimulatePhysics` (`self.Simulation Capsule`) true)
          (goto _label))))))