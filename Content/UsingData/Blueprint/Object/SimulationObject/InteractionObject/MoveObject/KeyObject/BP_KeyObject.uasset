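; BP_KeyObject is an interactable key, consumed when successfully used.
; Other objects register through Resister Animation Object, which adds them to the key's AnimationObject array.
; Interaction runs the parent interaction first; on success it calls UsingKey on every registered object, passing itself, then destroys the key and reports success.
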(fn `Interaction`
  (params (`Interaction Actor` :type "Actor Object Reference"))
  (returns (`Interaction Success` :type Boolean) (`Result Actor` :type "Actor Object Reference"))
  (bind _interaction_success (`parent.Interaction` `Interaction Actor`))
  (if _interaction_success
    (for _array_element (`self.Animation Object`)
      (`/Game/UsingData/Blueprint/Object/Non_SimulrationObject/Animation_Object/BP_AnimationObject.Using Key` _array_element self))
    (`self.K2_DestroyActor`)
    (return true null)))

(fn `Resister Animation Object`
  (params (`Animation Object` :type "/Game/UsingData/Blueprint/Object/Non_SimulrationObject/Animation_Object/BP_AnimationObject Object Reference"))
  (`KismetArrayLibrary.Array_Add` (`self.Animation Object`) `Animation Object`))

(fn `UserConstructionScript`
  (`parent.UserConstructionScript`))