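; Base gun weapon Blueprint that loads sockets, range, ammo and falling-object classes from a data asset by weapon name.
; Shot only checks ammo, messaging the owning character when empty, and ReLoad refills it.
; ShotTrace line-traces from the muzzle socket along camera forward for players or toward the current target for AI.
; Events spawn falling objects at sockets; SpawnFallingBullet uses the magazine class and adds a sideways impulse.
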(event `self.ReceiveBeginPlay`
  (bind (_result_weaponname _result_fallingbullet _result_fallingmagazine _result_magazinesocket _result_bulletsocket _result_shotsocket _result_attacklenght _result_remainbullet _result_maxbullet) (break `/Game/UsingData/Blueprint/Structure/Weapon/Gun/S_GuntypeInfo` (`/Game/UsingData/Blueprint/DataAsset/Weapon_GunInfoDataAsset/GunInfoDataAsset.Get GunInfo` (`self.Gun Info Data Asset`) (`self.Weapon Name`))))
  (`parent.ReceiveBeginPlay`)
  (set `self.Falling Bullet` _result_fallingbullet)
  (set `self.Falling Magazine` _result_fallingmagazine)
  (set `self.Magazine Socket` _result_magazinesocket)
  (set `self.Bullet Socket` _result_bulletsocket)
  (set `self.Shot Socket` _result_shotsocket)
  (set `self.Attack Lenght` _result_attacklenght)
  (set `self.Remain Bullet` _result_remainbullet)
  (set `self.Max Bullet` _result_maxbullet))

(event `/Game/UsingData/Blueprint/Interface/BPI_GunWeapon.Spawn Falling Magazine`
  (`|SpawnActorFromClass` (`self.Falling Magazine`) (`KismetMathLibrary.MakeTransform` (`SceneComponent.GetSocketLocation` (`self.SkeletalMesh`) (`self.Magazine Socket`))) "Undefined" "OverrideRootScale" null null))

(event `/Game/UsingData/Blueprint/Interface/BPI_GunWeapon.Spawn Falling Bullet`
  (bind _returnvalue (`|SpawnActorFromClass` (`self.Falling Magazine`) (`KismetMathLibrary.MakeTransform` (`SceneComponent.GetSocketLocation` (`self.SkeletalMesh`) (`self.Bullet Socket`))) "Undefined" "OverrideRootScale" null null))
  (bind _asbp_simulation_object (cast `/Game/UsingData/Blueprint/Object/SimulationObject/BP_SimulationObject` _returnvalue))
  (`self.Set Impulse` _asbp_simulation_object false 0.0 (`SceneComponent.GetRightVector` (`self.SkeletalMesh`)) (0.0 0.0 0.0)))

(fn `ReLoad`
  (returns (Success :type Boolean))
  (set `self.Remain Bullet` (`self.Max Bullet`))
  (return true))

(fn `Shot`
  (params (Succses :type Boolean))
  (returns (Succses_Shot :type Boolean))
  (if (> (`self.Remain Bullet`) 0)
    (return true)
    (else
      (bind _instigator (`self.Instigator`)
        (:`then`
          (bind _asbp_character (cast `/Game/UsingData/Blueprint/Character/BP_Character` _instigator))
          (message `/Game/UsingData/Blueprint/Interface/BPI_GunWeapon.ReLoad` _asbp_character)
          (return false))
        (:`else`)))))

(fn `Shot Trace`
  (params (Succses :type Boolean))
  (returns (Succsees :type Boolean) (`Out Hit` :type "HitResult Structure") (`Result Value` :type Boolean))
  (locals (`Shot StartPos` :type "Vector Structure") (`Shot EndPos` :type "Vector Structure"))
  (bind _instigator (`self.Instigator`))
  (if Succses
    (`|ExecutionSequence`
      (:`then_0`
        (set `local.Shot StartPos` (`SceneComponent.GetSocketLocation` (`self.SkeletalMesh`) (`self.Shot Socket`)))
        (cast `/Game/UsingData/Blueprint/Character/Player/BP_Player` _instigator
          (:`then`
            (set `local.Shot EndPos` (+ (* (`self.GetActorForwardVector` (`GameplayStatics.GetPlayerCameraManager` 0)) (`self.Attack Lenght`)) (`local.Shot StartPos`))))
          (:`CastFailed`
            (bind _asbp_aicharacter (cast `/Game/UsingData/Blueprint/Character/AICharacter/BP_AICharacter` _instigator))
            (bind _cur_target (`/Game/UsingData/Blueprint/Character/AICharacter/BP_AICharacter.Cur Target` _asbp_aicharacter)
              (:`then`
                (set `local.Shot EndPos` (+ (* (`KismetMathLibrary.Normal` (- (`self.K2_GetActorLocation` _cur_target) (`self.K2_GetActorLocation` _asbp_aicharacter))) (`self.Attack Lenght`)) (`local.Shot StartPos`))))
              (:`else`
                (return false (struct) false))))))
      (:`then_1`
        (bind (_outhit _returnvalue) (`KismetSystemLibrary.LineTraceSingle` (`local.Shot StartPos`) (`local.Shot EndPos`) "TraceTypeQuery3" false (`|MakeArray` (`self.GetInstigator`) :!type "Actor Object Reference") "ForDuration"))
        (return true _outhit _returnvalue)))))

(fn `UserConstructionScript`
  (`parent.UserConstructionScript`))