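; Main weapon pickup object that characters can interact with, carry and drop, with an optional paired weapon.
; Construction attaches the chosen mesh and weapon sockets to the selected simulation shape, and BeginPlay spawns the pair weapon.
; Pickup sets the instigator, disables simulation and applies per-character sockets from a data asset; dropping reverses this but requires a pair weapon.
; It also serves damage and per-character attack and skill montages.
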(event `self.ReceiveBeginPlay`
  (`parent.ReceiveBeginPlay`)
  (`ActorComponent.K2_DestroyComponent` (`self.StaticMesh Temp`))
  (`ActorComponent.K2_DestroyComponent` (`self.SkeletalMesh Temp`))
  (`|ExecutionSequence`
    (:`then_0`
      (bind _pair_weapon_class (`self.Pair Weapon Class`)
        (:`then`
          (bind _returnvalue (`|SpawnActorFromClass` _pair_weapon_class (`KismetMathLibrary.MakeTransform` (0.0 0.0 0.0)) "Undefined" "OverrideRootScale" null null))
          (bind _output_get (set `self.Pair Weapon` _returnvalue))
          (bind _asbp_pair_weapon (cast `/Game/UsingData/Blueprint/Object/Non_SimulrationObject/Pair_Weapon/BP_PairWeapon` _output_get))
          (`/Game/UsingData/Blueprint/Object/Non_SimulrationObject/Pair_Weapon/BP_PairWeapon.Dropping Pair Weapon` _asbp_pair_weapon self))
        (:`else`)))))

(fn `Activate`
  (params (success :type Boolean))
  (returns (Succsses :type Boolean))
  (return success))

(fn `Attach Pair Weapon To Main Weapon`
  (bind _asbp_pair_weapon (cast `/Game/UsingData/Blueprint/Object/Non_SimulrationObject/Pair_Weapon/BP_PairWeapon` (`self.Pair Weapon`)))
  (switch `/Game/UsingData/Blueprint/Enum/Object/E_MeshType` (`/Game/UsingData/Blueprint/Object/Non_SimulrationObject/BP_Non_SimulationObject.Mesh Type` _asbp_pair_weapon)
    (:`NewEnumerator1`
      (`SceneComponent.K2_AttachToComponent` (`/Game/UsingData/Blueprint/Object/Non_SimulrationObject/BP_Non_SimulationObject.StaticMesh` _asbp_pair_weapon) (`self.PairWeapon Socket`) "None" "KeepRelative" "KeepRelative" "KeepRelative" true))
    (:`NewEnumerator2`
      (`SceneComponent.K2_AttachToComponent` (`/Game/UsingData/Blueprint/Object/Non_SimulrationObject/BP_Non_SimulationObject.SkeletalMesh` _asbp_pair_weapon) (`self.PairWeapon Socket`) "None" "KeepRelative" "KeepRelative" "KeepRelative" true))))

(fn `Deactivate`
  (params (success :type Boolean))
  (returns (Succses :type Boolean))
  (return success))

(fn `DeAttach Actor`
  (locals (`Temp Location` :type "Vector Structure"))
  (bind _staticmesh (`self.StaticMesh`))
  (bind _skeletalmesh (`self.SkeletalMesh`))
  (switch `/Game/UsingData/Blueprint/Enum/Object/E_MeshType` (`self.MeshType`)
    (:`NewEnumerator1`
      (set `local.Temp Location` (`SceneComponent.K2_GetComponentLocation` _staticmesh))
      (`SceneComponent.K2_SetRelativeLocation` _staticmesh (0.0 0.0 0.0) false false))
    (:`NewEnumerator2`
      (set `local.Temp Location` (`SceneComponent.K2_GetComponentLocation` _skeletalmesh))
      (`SceneComponent.K2_SetRelativeLocation` _skeletalmesh (0.0 0.0 0.0) false false))))

(fn `Dropping Weapon`
  (returns (Success :type Boolean))
  (bind _asbp_pair_weapon (cast `/Game/UsingData/Blueprint/Object/Non_SimulrationObject/Pair_Weapon/BP_PairWeapon` (`self.Pair Weapon`))
    (:`then`
      (bind _success (`/Game/UsingData/Blueprint/Object/Non_SimulrationObject/Pair_Weapon/BP_PairWeapon.Dropping Pair Weapon` _asbp_pair_weapon self))
      (if _success
        (`self.Attach Pair Weapon To Main Weapon`)
        (`self.Set Simulation` true)
        (`self.Set Hidden OutLine` false)
        (set `self.Instigator` null)
        (`self.Set Scale` (`self.Weapon Scale`))
        (`self.Set Scale Mesh` (1.0 1.0 1.0))
        (`self.DeAttach Actor`)
        (`self.Set Interaction Collision` "QueryAndPhysics")
        (return true)
        (else
          _)))
    (:`CastFailed`
      _))
  (return false))

(fn `Get Damage`
  (returns (Damage :type "/Game/UsingData/Blueprint/Structure/Character/S_Hp_Update_value Structure"))
  (return (`self.Damage`)))

(fn `Get Montage Data`
  (params (`Character Name` :type "/Game/UsingData/Blueprint/Enum/Character/E_CharacterName Enum" :default "NewEnumerator0") (State :type "/Game/UsingData/Blueprint/Enum/Character/E_CharacterState Enum" :default "NewEnumerator0") (Combo :type Integer))
  (returns (Result :type "/Game/UsingData/Blueprint/Structure/S_MontageData Structure"))
  (return (`/Game/UsingData/Blueprint/DataAsset/MontageDataAsset/MontageDataAsset.Get Montage Data` (`BlueprintMapLibrary.Map_Find` (`self.Montage Data`) `Character Name`) State Combo)))

(fn `Get Skill Montage Data`
  (params (`Character Name` :type "/Game/UsingData/Blueprint/Enum/Character/E_CharacterName Enum" :default "NewEnumerator0") (`Skill Type` :type "/Game/UsingData/Blueprint/Enum/Weapon/E_SkillType Enum" :default "NewEnumerator0"))
  (returns (Result :type "/Game/UsingData/Blueprint/Structure/Weapon/S_WeaponSkillMontage Structure"))
  (return (`/Game/UsingData/Blueprint/DataAsset/MontageDataAsset/MontageDataAsset.Get Skill Montage Data` (`BlueprintMapLibrary.Map_Find` (`self.Montage Data`) `Character Name`) `Skill Type`)))

(fn `Interaction`
  (params (`Interaction Actor` :type "Actor Object Reference"))
  (returns (`Interaction Success` :type Boolean) (`Result Actor` :type "Actor Object Reference"))
  (bind (_interaction_success _result_actor) (`parent.Interaction` `Interaction Actor`))
  (if _interaction_success
    (bind _asbp_character (cast `/Game/UsingData/Blueprint/Character/BP_Character` _result_actor))
    (bind _can_pick_up_weapon (`/Game/UsingData/Blueprint/Character/BP_Character.Can Pick Up Weapon` _asbp_character (`self.Weapon Name`)))
    (if (and _can_pick_up_weapon (== (`self.GetInstigator`) null))
      (bind _success (`self.Pick Up Weapon` _result_actor))
      (if _success
        (return true self)))))

(fn `Pick Up Weapon`
  (params (Actor :type "Actor Object Reference"))
  (returns (Success :type Boolean))
  (bind _asbp_character (cast `/Game/UsingData/Blueprint/Character/BP_Character` Actor)
    (:`then`
      (bind _asbp_pair_weapon (cast `/Game/UsingData/Blueprint/Object/Non_SimulrationObject/Pair_Weapon/BP_PairWeapon` (`self.Pair Weapon`))
        (:`then`
          (bind _success (`/Game/UsingData/Blueprint/Object/Non_SimulrationObject/Pair_Weapon/BP_PairWeapon.Pick Up Pair Weapon` _asbp_pair_weapon _asbp_character))
          (if _success
            (set `self.Instigator` _asbp_character :!label _label)
            (`self.Set Equip To Character` false)
            (`self.Set Hidden OutLine` true)
            (`self.Set Simulation` false)
            (`self.Set Scale Mesh` (`self.Weapon Scale`))
            (`self.Set Interaction Collision` "NoCollision")
            (`self.Set Socket`)
            (return true)
            (else
              _)))
        (:`CastFailed`
          (goto _label))))
    (:`CastFailed`
      _))
  (return false))

(fn `Set Equip To Character`
  (params (Equip :type Boolean))
  (bind _asbp_character (cast `/Game/UsingData/Blueprint/Character/BP_Character` (`self.GetInstigator`)))
  (`/Game/UsingData/Blueprint/Character/BP_Character.Attach Actor To Character` _asbp_character self (`local.Equip`))
  (if (`local.Equip`)
    (`self.Set Visible` false)
    (else
      (`self.Set Visible` true))))

(fn `Set Socket`
  (bind _asbp_character (cast `/Game/UsingData/Blueprint/Character/BP_Character` (`self.GetInstigator`)))
  (bind _character_name (`/Game/UsingData/Blueprint/Character/BP_Character.Character Name` _asbp_character))
  (bind (_result_charactername _result_equipsocket _result_unequpsocket) (break `/Game/UsingData/Blueprint/Structure/Weapon/S_WeaponSocket` (`/Game/UsingData/Blueprint/DataAsset/WeaponSocketDataAsset/WeaponSocketDataAsset.Get Weapon Socket` (`self.SocketDataAsset`) false _character_name)))
  (set `self.Equip Socket` _result_equipsocket)
  (set `self.UnEquip Socket` _result_unequpsocket)
  (bind _asbp_pair_weapon (cast `/Game/UsingData/Blueprint/Object/Non_SimulrationObject/Pair_Weapon/BP_PairWeapon` (`self.Pair Weapon`)))
  (bind (_result_charactername_2 _result_equipsocket_2 _result_unequpsocket_2) (break `/Game/UsingData/Blueprint/Structure/Weapon/S_WeaponSocket` (`/Game/UsingData/Blueprint/DataAsset/WeaponSocketDataAsset/WeaponSocketDataAsset.Get Weapon Socket` (`self.SocketDataAsset`) true _character_name)))
  (set `/Game/UsingData/Blueprint/Object/Non_SimulrationObject/Pair_Weapon/BP_PairWeapon.Equip Socket` _result_equipsocket_2 _asbp_pair_weapon)
  (set `/Game/UsingData/Blueprint/Object/Non_SimulrationObject/Pair_Weapon/BP_PairWeapon.UnEquip Socket` _result_unequpsocket_2 _asbp_pair_weapon))

(fn `UserConstructionScript`
  (`parent.UserConstructionScript`)
  (`|ExecutionSequence`
    (:`then_0`
      (switch `/Game/UsingData/Blueprint/Enum/Object/E_MeshType` (`self.MeshType`)
        (:`NewEnumerator1`
          (`SceneComponent.K2_AttachToComponent` (`self.PairWeapon Socket`) (`self.StaticMesh`) "None" "KeepRelative" "KeepRelative" "KeepRelative" true))
        (:`NewEnumerator2`
          (`SceneComponent.K2_AttachToComponent` (`self.PairWeapon Socket`) (`self.SkeletalMesh`) "None" "KeepRelative" "KeepRelative" "KeepRelative" true))))
    (:`then_1`
      (switch `/Game/UsingData/Blueprint/Enum/Object/E_MeshType` (`self.MeshType`)
        (:`NewEnumerator1`
          (`SceneComponent.K2_AttachToComponent` (`self.StaticMesh`) (`self.Main Weapon Socket`) "None" "KeepRelative" "KeepRelative" "KeepRelative" true))
        (:`NewEnumerator2`
          (`SceneComponent.K2_AttachToComponent` (`self.SkeletalMesh`) (`self.Main Weapon Socket`) "None" "KeepRelative" "KeepRelative" "KeepRelative" true))))
    (:`then_2`
      (switch `/Game/UsingData/Blueprint/Enum/Object/E_SimulationType` (`self.Simulation Type`)
        (:`NewEnumerator4`
          (`SceneComponent.K2_AttachToComponent` (`self.Main Weapon Socket`) (`self.Simulation Box`) "None" "KeepRelative" "KeepRelative" "KeepRelative" true)
          (`SceneComponent.K2_AttachToComponent` (`self.PairWeapon Socket`) (`self.Simulation Box`) "None" "KeepRelative" "KeepRelative" "KeepRelative" true))
        (:`NewEnumerator5`
          (`SceneComponent.K2_AttachToComponent` (`self.Main Weapon Socket`) (`self.Simulation Sphere`) "None" "KeepRelative" "KeepRelative" "KeepRelative" true)
          (`SceneComponent.K2_AttachToComponent` (`self.PairWeapon Socket`) (`self.Simulation Sphere`) "None" "KeepRelative" "KeepRelative" "KeepRelative" true))
        (:`NewEnumerator6`
          (`SceneComponent.K2_AttachToComponent` (`self.Main Weapon Socket`) (`self.Simulation Capsule`) "None" "KeepRelative" "KeepRelative" "KeepRelative" true)
          (`SceneComponent.K2_AttachToComponent` (`self.PairWeapon Socket`) (`self.Simulation Capsule`) "None" "KeepRelative" "KeepRelative" "KeepRelative" true))))
    (:`then_3`
      (`self.Set Scale` (`self.Weapon Scale`)))))