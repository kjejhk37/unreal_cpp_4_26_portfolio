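; Dual blade melee weapon Blueprint that extends a parent weapon class to support a trail on its paired second blade.
; On BeginPlay, a valid PairWeapon is cast to BP_Pair_Melee_Weapon and PairTrail is attached to its StaticMesh.
; Activate and Deactivate call their parent versions; the BeginTrails call for PairTrail is disconnected, so this Blueprint never starts that trail.
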(event `self.ReceiveBeginPlay`
  (`parent.ReceiveBeginPlay`)
  (bind _pair_weapon (`self.Pair Weapon`)
    (:`then`
      (bind _asbp_pair_melee_weapon (cast `/Game/UsingData/Blueprint/Object/Non_SimulrationObject/Pair_Weapon/Melee/BP_Pair_Melee_Weapon` _pair_weapon))
      (`SceneComponent.K2_AttachToComponent` (`self.Pair_Trail`) (`/Game/UsingData/Blueprint/Object/Non_SimulrationObject/BP_Non_SimulationObject.StaticMesh` _asbp_pair_melee_weapon) "None" "KeepRelative" "KeepRelative" "KeepRelative" true))
    (:`else`)))

(fn `Activate`
  (params (success :type Boolean))
  (returns (Succsses :type Boolean))
  (bind _succsses (`parent.Activate` success)))

(fn `Deactivate`
  (params (success :type Boolean))
  (returns (Succses :type Boolean))
  (bind _succses (`parent.Deactivate` success))
  (return _succses))

(fn `UserConstructionScript`
  (`parent.UserConstructionScript`))