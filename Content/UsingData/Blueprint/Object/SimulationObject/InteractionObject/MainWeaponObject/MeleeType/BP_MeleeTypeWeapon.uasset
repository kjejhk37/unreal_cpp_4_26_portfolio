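; Melee main-weapon Blueprint that deals hits to characters and shows a weapon trail while active.
; The construction script attaches the chosen box, sphere or capsule hitbox and the trail particle to the static or skeletal mesh, destroying unused hitboxes.
; Hitbox overlaps with a BP_Character send it a damage message with the weapon as argument.
; Activate and Deactivate extend the parent functions to begin and end the socket-based trail.
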(event `self.Attack Collision Box.OnComponentBeginOverlap`
  (params (OverlappedComponent :type "PrimitiveComponent Object Reference") (OtherActor :type "Actor Object Reference") (OtherComp :type "PrimitiveComponent Object Reference") (OtherBodyIndex :type Integer) (bFromSweep :type Boolean) (SweepResult :type "HitResult Structure (by ref)"))
  (bind _asbp_character (cast `/Game/UsingData/Blueprint/Character/BP_Character` OtherActor))
  (message `/Game/UsingData/Blueprint/Interface/BPI_Character.Add Damage` _asbp_character self))

(event `self.Attack Collision Sphere.OnComponentBeginOverlap`
  (params (OverlappedComponent :type "PrimitiveComponent Object Reference") (OtherActor :type "Actor Object Reference") (OtherComp :type "PrimitiveComponent Object Reference") (OtherBodyIndex :type Integer) (bFromSweep :type Boolean) (SweepResult :type "HitResult Structure (by ref)"))
  (bind _asbp_character (cast `/Game/UsingData/Blueprint/Character/BP_Character` OtherActor))
  (message `/Game/UsingData/Blueprint/Interface/BPI_Character.Add Damage` _asbp_character self))

(event `self.Attack Collision Capsule.OnComponentBeginOverlap`
  (params (OverlappedComponent :type "PrimitiveComponent Object Reference") (OtherActor :type "Actor Object Reference") (OtherComp :type "PrimitiveComponent Object Reference") (OtherBodyIndex :type Integer) (bFromSweep :type Boolean) (SweepResult :type "HitResult Structure (by ref)"))
  (bind _asbp_character (cast `/Game/UsingData/Blueprint/Character/BP_Character` OtherActor))
  (message `/Game/UsingData/Blueprint/Interface/BPI_Character.Add Damage` _asbp_character self))

(event `self.Particle_DeActivate`
  (`ParticleSystemComponent.EndTrails` (`self.ParticleSystem`)))

(event `self.Particle_Activate`
  (`ParticleSystemComponent.BeginTrails` (`self.ParticleSystem`) (`self.Traill_Start_Socket`) (`self.Trail_End_Socket`) "ETrailWidthMode_FromCentre" 1.0))

(fn `Activate`
  (params (success :type Boolean))
  (returns (Succsses :type Boolean))
  (bind _succsses (`parent.Activate` success))
  (`self.Particle_Activate`)
  (return _succsses))

(fn `Deactivate`
  (params (success :type Boolean))
  (returns (Succses :type Boolean))
  (bind _succses (`parent.Deactivate` success))
  (`self.Particle_DeActivate`)
  (return _succses))

(fn `UserConstructionScript`
  (bind _attack_collision_type (`self.Attack Collision Type`))
  (`parent.UserConstructionScript`)
  (`|ExecutionSequence`
    (:`then_0`
      (switch `/Game/UsingData/Blueprint/Enum/Object/E_MeshType` (`self.MeshType`)
        (:`NewEnumerator1`
          (switch `/Game/UsingData/Blueprint/Enum/Object/E_CollsionType` _attack_collision_type
            (:`NewEnumerator1`
              (`SceneComponent.K2_AttachToComponent` (`self.Attack Collision Box`) (`self.StaticMesh`) "None" "KeepRelative" "KeepRelative" "KeepRelative" true))
            (:`NewEnumerator2`
              (`SceneComponent.K2_AttachToComponent` (`self.Attack Collision Sphere`) (`self.StaticMesh`) "None" "KeepRelative" "KeepRelative" "KeepRelative" true))
            (:`NewEnumerator3`
              (`SceneComponent.K2_AttachToComponent` (`self.Attack Collision Capsule`) (`self.StaticMesh`) "None" "KeepRelative" "KeepRelative" "KeepRelative" true))))
        (:`NewEnumerator2`
          (switch `/Game/UsingData/Blueprint/Enum/Object/E_CollsionType` _attack_collision_type
            (:`NewEnumerator1`
              (`SceneComponent.K2_AttachToComponent` (`self.Attack Collision Box`) (`self.SkeletalMesh`) "None" "KeepRelative" "KeepRelative" "KeepRelative" true))
            (:`NewEnumerator2`
              (`SceneComponent.K2_AttachToComponent` (`self.Attack Collision Sphere`) (`self.SkeletalMesh`) "None" "KeepRelative" "KeepRelative" "KeepRelative" true))
            (:`NewEnumerator3`
              (`SceneComponent.K2_AttachToComponent` (`self.Attack Collision Capsule`) (`self.SkeletalMesh`) "None" "KeepRelative" "KeepRelative" "KeepRelative" true))))))
    (:`then_1`
      (switch `/Game/UsingData/Blueprint/Enum/Object/E_CollsionType` (`self.Attack Collision Type`)
        (:`NewEnumerator1`
          (`ActorComponent.K2_DestroyComponent` (`self.Attack Collision Sphere`))
          (`ActorComponent.K2_DestroyComponent` (`self.Attack Collision Capsule`)))
        (:`NewEnumerator2`
          (`ActorComponent.K2_DestroyComponent` (`self.Attack Collision Box`))
          (`ActorComponent.K2_DestroyComponent` (`self.Attack Collision Capsule`)))
        (:`NewEnumerator3`
          (`ActorComponent.K2_DestroyComponent` (`self.Attack Collision Box`))
          (`ActorComponent.K2_DestroyComponent` (`self.Attack Collision Sphere`)))))
    (:`then_2`
      (switch `/Game/UsingData/Blueprint/Enum/Object/E_MeshType` (`self.MeshType`)
        (:`NewEnumerator0`
          (`ActorComponent.K2_DestroyComponent` (`self.ParticleSystem`)))
        (:`NewEnumerator1`
          (`SceneComponent.K2_AttachToComponent` (`self.ParticleSystem`) (`self.StaticMesh`) "None" "KeepRelative" "KeepRelative" "KeepRelative" true))
        (:`NewEnumerator2`
          (`SceneComponent.K2_AttachToComponent` (`self.ParticleSystem`) (`self.SkeletalMesh`) "None" "KeepRelative" "KeepRelative" "KeepRelative" true))))))