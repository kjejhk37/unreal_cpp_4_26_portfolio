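; BP_ItemObject is an interactable item that a character picks up into its inventory.
; Its Interaction override runs the parent check, then casts the resulting actor to BP_Character.
; The CanAddItem result for its ItemName feeds AddInventory along with the item itself; if that succeeds, the actor destroys itself and reports success.
; The event graph is unused, and the construction script only calls the parent.
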(fn `Interaction`
  (params (`Interaction Actor` :type "Actor Object Reference"))
  (returns (`Interaction Success` :type Boolean) (`Result Actor` :type "Actor Object Reference"))
  (bind (_interaction_success _result_actor) (`parent.Interaction` `Interaction Actor`))
  (if _interaction_success
    (bind _asbp_character (cast `/Game/UsingData/Blueprint/Character/BP_Character` _result_actor))
    (bind _can_add_item (`/Game/UsingData/Blueprint/Character/BP_Character.Can Add Item` _asbp_character (`self.Item Name`)))
    (bind _success (`/Game/UsingData/Blueprint/Character/BP_Character.Add Inventory` _asbp_character _can_add_item self))
    (if _success
      (`self.K2_DestroyActor`)
      (return true null))))

(fn `UserConstructionScript`
  (`parent.UserConstructionScript`))