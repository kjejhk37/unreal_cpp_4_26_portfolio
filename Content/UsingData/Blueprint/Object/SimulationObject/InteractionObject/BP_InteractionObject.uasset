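; Base interactable object that extends its parent with an interaction volume and an outline mesh.
; The construction script keeps the box, sphere or capsule chosen by InteractionType, attaches it to the static or skeletal mesh chosen by MeshType, and builds a matching outline copy with an outline material.
; Helper functions toggle outline visibility and interaction collision, while Interaction simply reports success and returns the passed-in actor.
; An unconnected branch for attaching to simulation shapes never runs.
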(fn `Interaction`
  (params (`Interaction Actor` :type "Actor Object Reference"))
  (returns (`Interaction Success` :type Boolean) (`Result Actor` :type "Actor Object Reference"))
  (return true `Interaction Actor`))

(fn `Set Hidden OutLine`
  (params (`New Hidden` :type Boolean))
  (bind _new_hidden (`local.New Hidden`))
  (switch `/Game/UsingData/Blueprint/Enum/Object/E_MeshType` (`self.MeshType`)
    (:`NewEnumerator1`
      (`SceneComponent.SetHiddenInGame` (`self.Outline Static Mesh`) _new_hidden false))
    (:`NewEnumerator2`
      (`SceneComponent.SetHiddenInGame` (`self.Outline Skeletal Mesh`) _new_hidden false))))

(fn `Set Interaction Collision`
  (params (`Collision Type` :type "ECollisionEnabled Enum" :default "NoCollision"))
  (switch `/Game/UsingData/Blueprint/Enum/Object/E_InteractionMeshType` (`self.Interaction Type`)
    (:`NewEnumerator1`
      (`PrimitiveComponent.SetCollisionEnabled` (`self.Interaction Box`) (`local.Collision Type`)))
    (:`NewEnumerator2`
      (`PrimitiveComponent.SetCollisionEnabled` (`self.Interaction Sphere`) (`local.Collision Type`)))
    (:`NewEnumerator3`
      (`PrimitiveComponent.SetCollisionEnabled` (`self.Interaction Capsule`) (`local.Collision Type`)))))

(fn `UserConstructionScript`
  (`parent.UserConstructionScript`)
  (`|ExecutionSequence`
    (:`then_0`
      (`|ExecutionSequence`
        (:`then_0`
          (switch `/Game/UsingData/Blueprint/Enum/Object/E_MeshType` (`self.MeshType`)
            (:`NewEnumerator1`
              (switch `/Game/UsingData/Blueprint/Enum/Object/E_InteractionMeshType` (`self.Interaction Type`)
                (:`NewEnumerator1`
                  (`SceneComponent.K2_AttachToComponent` (`self.Interaction Box`) (`self.StaticMesh`) "None" "KeepRelative" "KeepRelative" "KeepRelative" true))
                (:`NewEnumerator2`
                  (`SceneComponent.K2_AttachToComponent` (`self.Interaction Sphere`) (`self.StaticMesh`) "None" "KeepRelative" "KeepRelative" "KeepRelative" true))
                (:`NewEnumerator3`
                  (`SceneComponent.K2_AttachToComponent` (`self.Interaction Capsule`) (`self.StaticMesh`) "None" "KeepRelative" "KeepRelative" "KeepRelative" true))))
            (:`NewEnumerator2`
              (switch `/Game/UsingData/Blueprint/Enum/Object/E_InteractionMeshType` (`self.Interaction Type`)
                (:`NewEnumerator1`
                  (`SceneComponent.K2_AttachToComponent` (`self.Interaction Box`) (`self.SkeletalMesh`) "None" "KeepRelative" "KeepRelative" "KeepRelative" true))
                (:`NewEnumerator2`
                  (`SceneComponent.K2_AttachToComponent` (`self.Interaction Sphere`) (`self.SkeletalMesh`) "None" "KeepRelative" "KeepRelative" "KeepRelative" true))
                (:`NewEnumerator3`
                  (`SceneComponent.K2_AttachToComponent` (`self.Interaction Capsule`) (`self.SkeletalMesh`) "None" "KeepRelative" "KeepRelative" "KeepRelative" true))))))
        (:`then_1`
          (switch `/Game/UsingData/Blueprint/Enum/Object/E_InteractionMeshType` (`self.Interaction Type`)
            (:`NewEnumerator0`
              (`ActorComponent.K2_DestroyComponent` (`self.Interaction Box`))
              (`ActorComponent.K2_DestroyComponent` (`self.Interaction Sphere`))
              (`ActorComponent.K2_DestroyComponent` (`self.Interaction Capsule`)))
            (:`NewEnumerator1`
              (`ActorComponent.K2_DestroyComponent` (`self.Interaction Sphere`))
              (`ActorComponent.K2_DestroyComponent` (`self.Interaction Capsule`)))
            (:`NewEnumerator2`
              (`ActorComponent.K2_DestroyComponent` (`self.Interaction Box`))
              (`ActorComponent.K2_DestroyComponent` (`self.Interaction Capsule`)))
            (:`NewEnumerator3`
              (`ActorComponent.K2_DestroyComponent` (`self.Interaction Box`))
              (`ActorComponent.K2_DestroyComponent` (`self.Interaction Sphere`)))))))
    (:`then_1`
      (switch `/Game/UsingData/Blueprint/Enum/Object/E_MeshType` (`self.MeshType`)
        (:`NewEnumerator0`
          (`ActorComponent.K2_DestroyComponent` (`self.Outline Static Mesh`))
          (`ActorComponent.K2_DestroyComponent` (`self.Outline Skeletal Mesh`)))
        (:`NewEnumerator1`
          (`ActorComponent.K2_DestroyComponent` (`self.Outline Skeletal Mesh`))
          (`StaticMeshComponent.SetStaticMesh` (`self.Outline Static Mesh`) (`StaticMeshComponent.StaticMesh` (`self.StaticMesh`)))
          (`PrimitiveComponent.SetMaterial` (`self.Outline Static Mesh`) 0 "/Game/UsingData/Material/Outline/BPM_OutlineMaterail.BPM_OutlineMaterail")
          (`SceneComponent.K2_AttachToComponent` (`self.Outline Static Mesh`) (`self.StaticMesh`) "None" "KeepRelative" "KeepRelative" "KeepRelative" true))
        (:`NewEnumerator2`
          (`ActorComponent.K2_DestroyComponent` (`self.Outline Static Mesh`))
          (`SkinnedMeshComponent.SetSkinnedAssetAndUpdate` (`self.Outline Skeletal Mesh`) (`SkinnedMeshComponent.SkeletalMesh` (`self.SkeletalMesh`)) true)
          (`PrimitiveComponent.SetMaterial` (`self.Outline Skeletal Mesh`) 0 "/Game/UsingData/Material/Outline/BPM_OutlineMaterail.BPM_OutlineMaterail")
          (`SceneComponent.K2_AttachToComponent` (`self.Outline Skeletal Mesh`) (`self.SkeletalMesh`) "None" "KeepRelative" "KeepRelative" "KeepRelative" true))))))