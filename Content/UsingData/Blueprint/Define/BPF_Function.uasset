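; Blueprint function library, judging by its name, with helpers for camp hostility and local-to-world position conversion.
; GetHostile applies a one-directional rule table: Neutrality is hostile to nobody, Enemy to Neutrality and Player, and Player only to Enemy.
; GetActorLocalToWorld offsets an actor's location by LocalPosition along its forward, right and up vectors, ignoring actor scale.
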(fn `Get Actor Local To World`
  (params (Actor :type "Actor Object Reference") (`Local Position` :type "Vector Structure"))
  (returns (`World Position` :type "Vector Structure"))
  (return (+ (`Actor.K2_GetActorLocation` Actor) (* (`Actor.GetActorForwardVector` Actor) `Local Position_X`) (* (`Actor.GetActorRightVector` Actor) `Local Position_Y`) (* (`Actor.GetActorUpVector` Actor) `Local Position_Z`))))

(fn `Get hostile`
  (params (`My Camp` :type "/Game/UsingData/Blueprint/Enum/Camp/E_Camp Enum" :default "NewEnumerator0") (`Other Camp` :type "/Game/UsingData/Blueprint/Enum/Camp/E_Camp Enum" :default "NewEnumerator0"))
  (returns (`is Hostile` :type Boolean))
  (switch `/Game/UsingData/Blueprint/Enum/Camp/E_Camp` `My Camp`
    (:`NewEnumerator0`
      (switch `/Game/UsingData/Blueprint/Enum/Camp/E_Camp` `Other Camp`
        (:`NewEnumerator0`
          _)
        (:`NewEnumerator1`
          _)
        (:`NewEnumerator2`
          _)))
    (:`NewEnumerator1`
      (switch `/Game/UsingData/Blueprint/Enum/Camp/E_Camp` `Other Camp`
        (:`NewEnumerator0`
          (return true))
        (:`NewEnumerator1`
          _)
        (:`NewEnumerator2`
          (return true))))
    (:`NewEnumerator2`
      (switch `/Game/UsingData/Blueprint/Enum/Camp/E_Camp` `Other Camp`
        (:`NewEnumerator0`
          _)
        (:`NewEnumerator1`
          (return true))
        (:`NewEnumerator2`
          _))))
  (return false))