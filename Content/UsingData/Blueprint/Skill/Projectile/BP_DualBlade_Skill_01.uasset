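; Skill projectile Blueprint for the first Dual Blade skill, built on a parent class that supplies the base Play behavior.
; The Play override calls the parent, then SetPointersToWorldPos, and returns false if that fails.
; On success it spawns meshes, resets skill time and index, zeroes projectile velocity, flags playing and delay, and shows the particle system.
; The event graph and construction script add no logic of their own.
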(fn `Play`
  (params (`Success in` :type Boolean))
  (returns (`Success out` :type Boolean))
  (`parent.Play` `Success in`)
  (bind _success (`self.Set Pointers To World Pos`))
  (if _success
    (`self.Spawns Meshs`)
    (set `self.is Play` true)
    (set `self.Cur Time` 0.0)
    (set `self.Cur Skill Index` 0)
    (set `MovementComponent.Velocity` (0.0 0.0 0.0) (`self.ProjectileMovement`))
    (set `self.is Delay` true)
    (`SceneComponent.SetVisibility` (`self.ParticleSystem`) true false)
    (return true)
    (else
      (return false))))

(fn `UserConstructionScript`
  (`parent.UserConstructionScript`))