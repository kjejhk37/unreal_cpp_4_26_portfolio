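; Base skill projectile that flies through a chain of waypoints, pausing before each leg, then destroys itself with a grenade explosion effect.
; SetPointersToWorldPos converts actor-local points to world positions and derives each leg's travel time from the initial speed.
; SpawnsMeshs places an actor at each waypoint, yawed along its leg.
; Once IsPlay is set, Tick alternates timed delays and constant-velocity moves, removing waypoint actors along the way.
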(event `self.ReceiveTick`
  (params (DeltaSeconds :type "Float (single-precision)"))
  (`parent.ReceiveTick` DeltaSeconds)
  (if (`self.is Play`)
    (bind _output_get (set `self.Cur Time` (+ DeltaSeconds (`self.Cur Time`))))
    (if (`self.is Delay`)
      (if (>= _output_get (`|GetArrayItem` (`self.Delay Times`) (`self.Cur Skill Index`)))
        (set `self.is Delay` false)
        (set `self.Cur Time` 0.0)
        (`self.Set Velocity` (`self.Cur Skill Index`))
        (`SceneComponent.SetVisibility` (`self.ParticleSystem`) true false)
        (if (not (== (`self.Cur Skill Index`) 0))
          (`self.K2_DestroyActor` (`|GetArrayItem` (`self.Meshs`) (- (`self.Cur Skill Index`) 1)))))
      (elif (>= _output_get (`|GetArrayItem` (`self.Times`) (`self.Cur Skill Index`)))
        (if (== (`self.Cur Skill Index`) (- (`KismetArrayLibrary.Array_Length` (`self.Times`)) 1))
          (`self.K2_DestroyActor` (`|GetArrayItem` (`self.Meshs`) (`self.Cur Skill Index`)))
          (`self.K2_DestroyActor`)
          (`GameplayStatics.SpawnEmitterAtLocation` "/Game/UsingData/Weapon/FX/P_Grenade_Explosion_01.P_Grenade_Explosion_01" (- (`self.K2_GetActorLocation`) (0.0 0.0 90.0)) (`self.K2_GetActorRotation`))
          (else
            (`/Engine/EditorBlueprintResources/StandardMacros.IncrementInt` (`self.Cur Skill Index`)
              (:`  `
                (set `self.Cur Time` 0.0)
                (set `self.is Delay` true)
                (set `MovementComponent.Velocity` (0.0 0.0 0.0) (`self.ProjectileMovement`))
                (`SceneComponent.SetVisibility` (`self.ParticleSystem`) true false)))))))))

(fn `Play`
  (params (`Success in` :type Boolean))
  (returns (`Success out` :type Boolean))
  (return `Success in`))

(fn `Set Pointers To World Pos`
  (returns (Success :type Boolean))
  (bind _world_positions (`self.World Positions`))
  (bind _initialspeed (`ProjectileMovementComponent.InitialSpeed` (`self.ProjectileMovement`)))
  (`KismetArrayLibrary.Array_Clear` (`self.Times`))
  (`KismetArrayLibrary.Array_Clear` (`self.World Positions`))
  (for (_array_element _array_index) (`self.Local Pointers`)
    (bind _returnvalue (+ (* (`self.GetActorUpVector`) (.z _array_element)) (* (`self.GetActorRightVector`) (.y _array_element)) (* (`self.GetActorForwardVector`) (.x _array_element)) (`self.K2_GetActorLocation`)))
    (`KismetArrayLibrary.Array_Add` _world_positions _returnvalue)
    (if (== _array_index 0)
      (`KismetArrayLibrary.Array_Add` (`self.Times`) (/ (`KismetMathLibrary.VSize` (- (`self.K2_GetActorLocation`) _returnvalue)) _initialspeed))
      (else
        (`KismetArrayLibrary.Array_Add` (`self.Times`) (/ (`KismetMathLibrary.VSize` (- (`|GetArrayItem` _world_positions (- _array_index 1)) _returnvalue)) _initialspeed)))))
  (return (> (`KismetArrayLibrary.Array_Length` (`self.World Positions`)) 0)))

(fn `Set Velocity`
  (params (`Skill Index` :type Integer))
  (locals (`Start Position` :type "Vector Structure") (`End Position` :type "Vector Structure"))
  (bind _projectilemovement (`self.ProjectileMovement`))
  (set `local.End Position` (`|GetArrayItem` (`self.World Positions`) `Skill Index`))
  (if (== `Skill Index` 0)
    (set `local.Start Position` (`self.K2_GetActorLocation`))
    (else
      (set `local.Start Position` (`|GetArrayItem` (`self.World Positions`) (- `Skill Index` 1)))))
  (set `MovementComponent.Velocity` (* (`KismetMathLibrary.Normal` (- (`local.End Position`) (`local.Start Position`))) (`ProjectileMovementComponent.InitialSpeed` _projectilemovement)) _projectilemovement))

(fn `Spawns Meshs`
  (locals (`Spawn Transform Rotation` :type "Float (double-precision)"))
  (bind _world_positions (`self.World Positions`))
  (for (_array_element _array_index) (`self.MeshTypes`)
    (if (== _array_index 0)
      (bind _output (`|GetArrayItem` _world_positions _array_index))
      (bind (_returnvalue_roll _returnvalue_pitch _returnvalue_yaw) (`KismetMathLibrary.BreakRotator` (`KismetMathLibrary.FindLookAtRotation` (`self.K2_GetActorLocation`) _output)))
      (set `local.Spawn Transform Rotation` _returnvalue_yaw)
      (else
        (bind (_returnvalue_roll_2 _returnvalue_pitch_2 _returnvalue_yaw_2) (`KismetMathLibrary.BreakRotator` (`KismetMathLibrary.FindLookAtRotation` (`|GetArrayItem` _world_positions (- _array_index 1)) _output)))
        (set `local.Spawn Transform Rotation` _returnvalue_yaw_2)))
    (bind _returnvalue (`|SpawnActorFromClass` _array_element (`KismetMathLibrary.MakeTransform` (- _output (0.0 0.0 90.0)) (`KismetMathLibrary.MakeRotator` 0.0 0.0 (- (`local.Spawn Transform Rotation`) 90.0))) "Undefined" "OverrideRootScale" null null))
    (`KismetArrayLibrary.Array_Add` (`self.Meshs`) _returnvalue)))

(fn `UserConstructionScript`)