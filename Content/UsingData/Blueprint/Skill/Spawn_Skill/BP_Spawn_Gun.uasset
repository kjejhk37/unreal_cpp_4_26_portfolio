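; BP_Spawn_Gun is a spawned skill actor: a floating gun that fires a set number of shots, then rises away and destroys itself.
; Tick bobs it around its start position with sine offsets, holding a rotation that LookAtTarget aims at the target character's center.
; Play starts a delayed montage loop, with CheckEnd counting down shots.
; GunShot line-traces forward from the muzzle socket with debug drawing, leaving the hit unused.
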(event `self.ReceiveBeginPlay`
  (`parent.ReceiveBeginPlay`))

(event `self.ReceiveTick`
  (params (DeltaSeconds :type "Float (single-precision)"))
  (`parent.ReceiveTick` DeltaSeconds)
  (bind _output_get (set `self.Play Time` (+ DeltaSeconds (`self.Play Time`))))
  (`self.K2_SetActorLocationAndRotation` (+ (`self.World Start Position`) (`KismetMathLibrary.MakeVector` 0.0 (* (`KismetMathLibrary.Sin` (* _output_get 1.5)) 50.0) (* (`KismetMathLibrary.Sin` (* _output_get 0.75)) 60.0))) (`self.Start Rotation`))
  (if (`self.End Play`)
    (bind _output_get_2 (set `self.EndPlay Time` (+ (`self.EndPlay Time`) DeltaSeconds)))
    (`self.K2_SetActorLocation` (+ (`self.K2_GetActorLocation`) (`KismetMathLibrary.MakeVector` 0.0 0.0 (* _output_get_2 (`self.EndPlay Speed`)))) false true)))

(event `Shot`
  (params (`is Delay` :type Boolean))
  (if `is Delay`
    (`KismetSystemLibrary.Delay` (`self.Delay Time`)))
  (`|PlayMontage` (`self.SkeletalMesh`) "/Game/CBP_Data/BP/Skill/Skill_Animation/Fire_Spawn_Gun_Montage.Fire_Spawn_Gun_Montage" (* (`self.Attack Cool Time`) 5.0)
    (:`OnCompleted`
      (`self.Check End`))))

(event `Set End`
  (`KismetSystemLibrary.Delay` 1.0)
  (set `self.End Play` true)
  (`KismetSystemLibrary.Delay` 3.0)
  (`self.K2_DestroyActor`))

(fn `Check End`
  (if (`self.Stop Shot`)
    (set `self.Stop Shot` false)
    (else
      (bind _result (`/Engine/EditorBlueprintResources/StandardMacros.DecrementInt` (`self.Attack Count`))
        (:`  `
          (if (<= _result 0)
            (`self.Set End`)
            (else
              (`self.Shot` false))))))))

(fn `Gun_Shot`
  (bind _returnvalue (`SceneComponent.GetSocketLocation` (`self.SkeletalMesh`) "Shot"))
  (`KismetSystemLibrary.LineTraceSingle` _returnvalue (+ _returnvalue (* (`self.GetActorForwardVector`) (`self.Attack length`))) "TraceTypeQuery3" false (`|MakeArray` (`self.GetInstigator`) :!type "Actor Object Reference") "ForDuration"))

(fn `Look At Target`
  (bind _asbp_character (cast `/Game/UsingData/Blueprint/Character/BP_Character` (`self.Target`)))
  (set `self.Start Rotation` (`KismetMathLibrary.FindLookAtRotation` (`self.World Start Position`) (`SceneComponent.K2_GetComponentLocation` (`/Game/UsingData/Blueprint/Character/BP_Character.CharacterCenter` _asbp_character)))))

(fn `Play`
  (params (`Success in` :type Boolean))
  (returns (`Success out` :type Boolean))
  (`parent.Play` `Success in`)
  (`self.Shot` true)
  (return true))

(fn `UserConstructionScript`
  (`parent.UserConstructionScript`))