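; Base character Blueprint handling combat, weapon equipping, charged jumps, inventory, skills and health, with a camp hostility check on damage.
; A CharacterState enum gates actions through Can* checks.
; Weapons supply montage data per character, with montage notifies driving combo windows, weapon activation, trails and socket attach swaps.
; Damage enters a queue that a pausable timer handler applies to HP, setting Dead at zero.
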(event `self.ReceiveBeginPlay`
  (bind (_result_charactername _result_maxhp _result_maxweaponinventorynum _result_maxiteminventorynum) (break `/Game/UsingData/Blueprint/Structure/Character/S_CharacterInfo` (`/Game/UsingData/Blueprint/DataAsset/CharacterInfoDataAsset/CharacterInfoDataAsset.Get Character Data` (`self.Character Data Asset`) (`self.Character Name`))))
  (`parent.ReceiveBeginPlay`)
  (`|ExecutionSequence`
    (:`then_0`
      (set `self.Max_Hp` _result_maxhp)
      (set `self.Max Weapon Inventory Num` _result_maxweaponinventorynum)
      (set `self.Max Item Inventory Num` _result_maxiteminventorynum)
      (set `self.Cur_Hp` (`self.Max_Hp`)))
    (:`then_1`
      (bind _returnvalue (`KismetSystemLibrary.K2_SetTimerDelegate` (delegate `Update Hp`) 0.1))
      (bind _output_get (set `self.Hp_Update_Handle` _returnvalue))
      (`KismetSystemLibrary.K2_PauseTimerHandle` _output_get))))

(event `Update Hp`
  (`self.Update Hp Value`))

(event `self.ReSetState`
  (set `self.Character State` "NewEnumerator0")
  (set `self.Attack Count` 0)
  (set `self.Cur Attack Is End` true))

(event `self.ReceiveTick`
  (params (DeltaSeconds :type "Float (single-precision)"))
  (bind (_jump_data_charactername _jump_data_minjumppower _jump_data_max_jumppower _jump_data_charge) (break `/Game/UsingData/Blueprint/Structure/Character/S_JumpData` (`self.Jump Data`)))
  (if (`self.is Jump ready`)
    (set `self.Cur Jump Power` (`KismetMathLibrary.FClamp` (+ (`self.Cur Jump Power`) (* DeltaSeconds _jump_data_charge)) _jump_data_minjumppower _jump_data_max_jumppower))
    (else
      (set `self.Cur Jump Power` 0.0))))

(event `self.Action`
  (bind _main_weapon (`self.Main Weapon`))
  (bind (_temp_montage_data_state _temp_montage_data_combo _temp_montage_data_montagedata _temp_montage_data_playrate _temp_montage_data_startname _temp_montage_data_nextcombo) (break `/Game/UsingData/Blueprint/Structure/S_MontageData` (`self.Temp Montage Data`)))
  (bind _pair_weapon (`self.Pair Weapon`))
  (`self.Main Weapon`
    (:`then`
      (bind _can_attack (`self.Can Attack`))
      (if _can_attack
        (set `self.Character State` "NewEnumerator4")
        (bind _asbp_weapon_object (cast `/Game/UsingData/Blueprint/Object/SimulationObject/InteractionObject/MainWeaponObject/BP_WeaponObject` (`self.Main Weapon`)))
        (bind _output_get (set `self.Temp Montage Data` (`/Game/UsingData/Blueprint/Object/SimulationObject/InteractionObject/MainWeaponObject/BP_WeaponObject.Get Montage Data` _asbp_weapon_object (`self.Character Name`) (`self.Character State`) (`self.Attack Count`)) :!label _label))
        (bind _notifyname (`|PlayMontage` (`self.Mesh`) (`.MontageData_5_A0D7BF334975575F779FBD9E837F7BC1` (break `/Game/UsingData/Blueprint/Structure/S_MontageData` _output_get)) (`.Playrate_7_9EC5A6E84111D8C1223B4D8846CF0B7A` (break `/Game/UsingData/Blueprint/Structure/S_MontageData` _output_get)) 0.0 (`.StartName_9_2B59D29146FD2A75BBB652AB06A981D6` (break `/Game/UsingData/Blueprint/Structure/S_MontageData` _output_get)))
          (:`then`
            (`/Engine/EditorBlueprintResources/StandardMacros.IncrementInt` (`self.Attack Count`)) ; 더해
          )
          (:`OnCompleted`
            (`self.ReSetState`))
          (:`OnBlendOut`
            (if (not (`self.Cur Attack Is End`))
              (set `self.Cur Attack Is End` true)
              (goto _label)))
          (:`OnNotifyBegin`
            (switch `name` _notifyname
              (:`EnableNextAttack`
                (set `self.Enable Next Attack` true))
              (:`UnEnableNextAttack`
                (set `self.Enable Next Attack` false))
              (:`Main_Weapon_Activate`
                (message `/Game/UsingData/Blueprint/Interface/BPI_Weapon.Activate` _main_weapon true))
              (:`Main_Weapon_DeActivate`
                (message `/Game/UsingData/Blueprint/Interface/BPI_Weapon.Deactivate` _main_weapon true))
              (:`Pair_Weapon_Activate`
                (message `/Game/UsingData/Blueprint/Interface/BPI_Weapon.Activate` _pair_weapon true))
              (:`Pair_Weapon_DeActivate`
                (message `/Game/UsingData/Blueprint/Interface/BPI_Weapon.Deactivate` _pair_weapon true))
              (:`Trail_Activate`
                (message `/Game/UsingData/Blueprint/Interface/BPI_Trail_Particle_Weapon.Particle_Activate` (`self.Main Weapon`))
                (message `/Game/UsingData/Blueprint/Interface/BPI_Trail_Particle_Weapon.Particle_Activate` (`self.Pair Weapon`)))
              (:`Trail_DeActivate`
                (message `/Game/UsingData/Blueprint/Interface/BPI_Trail_Particle_Weapon.Particle_DeActivate` (`self.Main Weapon`))
                (message `/Game/UsingData/Blueprint/Interface/BPI_Trail_Particle_Weapon.Particle_DeActivate` (`self.Pair Weapon`))))))
        (elif (`self.Is Character State` "NewEnumerator4")
          (if (and _temp_montage_data_nextcombo (`self.Enable Next Attack`))
            (set `self.Cur Attack Is End` false)))))
    (:`else`)))

(event `self.Equp Or UnEquip`
  (bind _can_armming (`self.Can Armming`))
  (if _can_armming
    (`|ExecutionSequence`
      (:`then_0`
        (bind _main_weapon (`self.Main Weapon`)
          (:`then`
            (if (== (`|GetArrayItem` (`self.Weapon Inventory`) (`self.Cur Using Weapon Num`)) _main_weapon)
              (set `self.Character State` "NewEnumerator26")
              (else
                (set `self.Character State` "NewEnumerator27"))))
          (:`else`
            (set `self.Character State` "NewEnumerator27"))))
      (:`then_1`
        (if (`self.Is Character State` "NewEnumerator26")
          (bind _asbp_weapon_object (cast `/Game/UsingData/Blueprint/Object/SimulationObject/InteractionObject/MainWeaponObject/BP_WeaponObject` (`self.Main Weapon`)))
          (bind (_result_state _result_combo _result_montagedata _result_playrate _result_startname) (break `/Game/UsingData/Blueprint/Structure/S_MontageData` (`/Game/UsingData/Blueprint/Object/SimulationObject/InteractionObject/MainWeaponObject/BP_WeaponObject.Get Montage Data` _asbp_weapon_object (`self.Character Name`) (`self.Character State`) 0)))
          (bind _notifyname (`|PlayMontage` (`self.Mesh`) _result_montagedata _result_playrate 0.0 _result_startname)
            (:`OnCompleted`
              (`self.ReSetState`))
            (:`OnNotifyBegin`
              (switch `name` _notifyname
                (:`Equip`
                  (`self.Attach Actor To Character` (`self.Main Weapon`))
                  (`self.Attach Actor To Character` (`self.Pair Weapon`))
                  (set `self.Main Weapon` null)
                  (set `self.Pair Weapon` null)))))
          (else
            (bind _asbp_weapon_object_2 (cast `/Game/UsingData/Blueprint/Object/SimulationObject/InteractionObject/MainWeaponObject/BP_WeaponObject` (`|GetArrayItem` (`self.Weapon Inventory`) (`self.Cur Using Weapon Num`))))
            (bind (_result_state_2 _result_combo_2 _result_montagedata_2 _result_playrate_2 _result_startname_2) (break `/Game/UsingData/Blueprint/Structure/S_MontageData` (`/Game/UsingData/Blueprint/Object/SimulationObject/InteractionObject/MainWeaponObject/BP_WeaponObject.Get Montage Data` _asbp_weapon_object_2 (`self.Character Name`) (`self.Character State`) 0)))
            (bind _notifyname_2 (`|PlayMontage` (`self.Mesh`) _result_montagedata_2 _result_playrate_2 0.0 _result_startname_2)
              (:`OnCompleted`
                (`self.ReSetState`))
              (:`OnNotifyBegin`
                (switch `name` _notifyname_2
                  (:`Equip`
                    (`self.Main Weapon`
                      (:`then`
                        (`self.Attach Actor To Character` (`self.Main Weapon`))
                        (`self.Attach Actor To Character` (`self.Pair Weapon`)))
                      (:`else`
                        _))
                    (bind _output_get (set `self.Main Weapon` (`|GetArrayItem` (`self.Weapon Inventory`) (`self.Cur Using Weapon Num`))))
                    (bind _asbp_weapon_object_3 (cast `/Game/UsingData/Blueprint/Object/SimulationObject/InteractionObject/MainWeaponObject/BP_WeaponObject` _output_get))
                    (bind _output_get_2 (set `self.Pair Weapon` (`/Game/UsingData/Blueprint/Object/SimulationObject/InteractionObject/MainWeaponObject/BP_WeaponObject.Pair Weapon` _asbp_weapon_object_3)))
                    (`self.Attach Actor To Character` _output_get true)
                    (`self.Attach Actor To Character` _output_get_2 true)))))))))))

(event `self.Skill`
  (params (`Skill Type` :type "/Game/UsingData/Blueprint/Enum/Weapon/E_SkillType Enum" :default "NewEnumerator0"))
  (bind _skill_cool_time (`self.Skill Cool Time`))
  (bind _can_skill (`self.Can Action Skill` `Skill Type`))
  (if _can_skill
    (set `self.Character State` "NewEnumerator30")
    (bind _asbp_weapon_object (cast `/Game/UsingData/Blueprint/Object/SimulationObject/InteractionObject/MainWeaponObject/BP_WeaponObject` (`self.Main Weapon`)))
    (bind (_result_skilltype _result_montage _result_playrate _result_sectionname _result_cooltime) (break `/Game/UsingData/Blueprint/Structure/Weapon/S_WeaponSkillMontage` (`/Game/UsingData/Blueprint/Object/SimulationObject/InteractionObject/MainWeaponObject/BP_WeaponObject.Get Skill Montage Data` _asbp_weapon_object (`self.Character Name`) `Skill Type`)))
    (bind _notifyname (`|PlayMontage` (`self.Mesh`) _result_montage _result_playrate 0.0 _result_sectionname)
      (:`then`
        (`BlueprintMapLibrary.Map_Add` _skill_cool_time `Skill Type`)
        (`KismetSystemLibrary.RetriggerableDelay` _result_cooltime)
        (`BlueprintMapLibrary.Map_Add` _skill_cool_time `Skill Type` true))
      (:`OnCompleted`
        (`self.ReSetState`))
      (:`OnNotifyBegin`
        (switch `name` _notifyname))
      (:`OnNotifyEnd`
        (switch `name` _notifyname)))))

(event `Skill Start`
  (params (`Skill Class` :type "/Game/UsingData/Blueprint/Skill/Projectile/BP_Skill_PeojectileBase Class Reference"))
  (bind (_returnvalue_roll _returnvalue_pitch _returnvalue_yaw) (`KismetMathLibrary.BreakRotator` (`self.K2_GetActorRotation`)))
  (bind _returnvalue (`|SpawnActorFromClass` `Skill Class` (`KismetMathLibrary.MakeTransform` (`self.K2_GetActorLocation`) (`KismetMathLibrary.MakeRotator` 0.0 0.0 _returnvalue_yaw)) "Undefined" "OverrideRootScale" self self))
  (`/Game/UsingData/Blueprint/Skill/Projectile/BP_Skill_PeojectileBase.Play` _returnvalue true))

(event `Skill End`)

(event `self.Weapon_Select`
  (params (`inventory Num` :type Integer))
  (if (> (`KismetArrayLibrary.Array_Length` (`self.Weapon Inventory`)) `inventory Num`)
    (set `self.Cur Using Weapon Num` `inventory Num`)
    (`self.Equp Or UnEquip`)))

(event `self.Speaker`)

(event `self.Character Crouch`
  (params (Crouch :type Boolean)))

(event `self.Character Jump`
  (params (`is Jump` :type Boolean))
  (bind _can_jump (`self.Can Jump`))
  (if _can_jump
    (if (and (== `is Jump` true) (== (`self.is Jump ready`) false))
      (set `self.is Jump ready` true)
      (elif (and (== `is Jump` false) (== (`self.is Jump ready`) true))
        (set `CharacterMovementComponent.JumpZVelocity` (`self.Cur Jump Power`) (`self.CharacterMovement`))
        (set `self.is Jump ready` false)
        (set `self.Character State` "NewEnumerator28")
        (`self.Jump`)))))

(event `Jump Start`
  (`self.Main Weapon`
    (:`then`
      (`|PlayMontage` null))
    (:`else`
      (`|PlayMontage` null))))

(event `Jump End`
  (`self.Main Weapon`
    (:`then`
      (`|PlayMontage` null))
    (:`else`
      (`|PlayMontage` null
        (:`then`
          (`self.ReSetState`))))))

(event `self.Zoom Camera Out`
  (`Timeline|타임라인_0` :!label _label))

(event `self.Zoom Camera In`
  (goto _label :!via `Reverse`))

(fn `Action Dropping`
  (returns (Success :type Boolean))
  (return true))

(fn `Add Damage`
  (params (`Weapon Actor` :type "Actor Object Reference"))
  (returns (Success :type Boolean))
  (bind _asbp_weapon_object (cast `/Game/UsingData/Blueprint/Object/SimulationObject/InteractionObject/MainWeaponObject/BP_WeaponObject` `Weapon Actor`))
  (bind _asbp_character (cast `/Game/UsingData/Blueprint/Character/BP_Character` (`self.GetInstigator` _asbp_weapon_object)))
  (if (`/Game/UsingData/Blueprint/Define/BPF_Function.Get hostile` (`self.Camp`) (`/Game/UsingData/Blueprint/Character/BP_Character.Camp` _asbp_character))
    (bind (_damage_float _damage_int _damage_int2 _damage_int3) (break `/Game/UsingData/Blueprint/Structure/Character/S_Hp_Update_value` (`/Game/UsingData/Blueprint/Object/SimulationObject/InteractionObject/MainWeaponObject/BP_WeaponObject.Get Damage` _asbp_weapon_object)))
    (`self.Add Hp Update` _damage_float _damage_int _damage_int2 _damage_int3)
    (return true)))

(fn `Add Hp Update`
  (params (Value :type "Float (double-precision)") (Count :type Integer) (Temp :type Integer) (`Temp Max` :type Integer))
  (`KismetArrayLibrary.Array_Add` (`self.HP_Value_Vector`) (make `/Game/UsingData/Blueprint/Structure/Character/S_Hp_Update_value` Value Count Temp `Temp Max`))
  (if (`KismetSystemLibrary.K2_IsTimerPausedHandle` (`self.Hp_Update_Handle`))
    (`KismetSystemLibrary.K2_UnPauseTimerHandle` (`self.Hp_Update_Handle`))))

(fn `Add Inventory`
  (params (Result :type Boolean) (Actor :type "Actor Object Reference"))
  (returns (Success :type Boolean))
  (bind _item_inventory (`self.Item Inventory`))
  (if Result
    (bind _asbp_weapon_object (cast `/Game/UsingData/Blueprint/Object/SimulationObject/InteractionObject/MainWeaponObject/BP_WeaponObject` Actor)
      (:`then`
        (`KismetArrayLibrary.Array_Add` (`self.Weapon Inventory`) _asbp_weapon_object)
        (return true))
      (:`CastFailed`
        (bind _asbp_item_object (cast `/Game/UsingData/Blueprint/Object/SimulationObject/InteractionObject/ItemObject/BP_ItemObject` Actor))
        (bind _item_name (`/Game/UsingData/Blueprint/Object/SimulationObject/InteractionObject/ItemObject/BP_ItemObject.Item Name` _asbp_item_object))
        (`BlueprintMapLibrary.Map_Add` _item_inventory _item_name (+ (`BlueprintMapLibrary.Map_Find` _item_inventory _item_name) (`/Game/UsingData/Blueprint/Object/SimulationObject/InteractionObject/ItemObject/BP_ItemObject.Item Num` _asbp_item_object)))
        (return true)))))

(fn `Attach Actor To Character`
  (params (Actor :type "Actor Object Reference") (Equip :type Boolean))
  (locals (Socket :type Name))
  (bind _returnvalue (not (`local.Equip`)))
  (`|ExecutionSequence`
    (:`then_0`
      (bind _asbp_weapon_object (cast `/Game/UsingData/Blueprint/Object/SimulationObject/InteractionObject/MainWeaponObject/BP_WeaponObject` Actor)
        (:`then`
          (if (`local.Equip`)
            (set `local.Socket` (`/Game/UsingData/Blueprint/Object/SimulationObject/InteractionObject/MainWeaponObject/BP_WeaponObject.Equip Socket` _asbp_weapon_object))
            (else
              (set `local.Socket` (`/Game/UsingData/Blueprint/Object/SimulationObject/InteractionObject/MainWeaponObject/BP_WeaponObject.UnEquip Socket` _asbp_weapon_object))))
          (switch `/Game/UsingData/Blueprint/Enum/Object/E_MeshType` (`/Game/UsingData/Blueprint/Object/SimulationObject/BP_SimulationObject.MeshType` _asbp_weapon_object)
            (:`NewEnumerator1`
              (`SceneComponent.K2_AttachToComponent` (`/Game/UsingData/Blueprint/Object/SimulationObject/BP_SimulationObject.StaticMesh` _asbp_weapon_object) (`self.Mesh`) (`local.Socket`) "KeepRelative" "KeepRelative" "KeepRelative" true))
            (:`NewEnumerator2`
              (`SceneComponent.K2_AttachToComponent` (`/Game/UsingData/Blueprint/Object/SimulationObject/BP_SimulationObject.SkeletalMesh` _asbp_weapon_object) (`self.Mesh`) (`local.Socket`) "KeepRelative" "KeepRelative" "KeepRelative" true))))
        (:`CastFailed`
          (bind _asbp_pair_weapon (cast `/Game/UsingData/Blueprint/Object/Non_SimulrationObject/Pair_Weapon/BP_PairWeapon` Actor))
          (if (`local.Equip`)
            (set `local.Socket` (`/Game/UsingData/Blueprint/Object/Non_SimulrationObject/Pair_Weapon/BP_PairWeapon.Equip Socket` _asbp_pair_weapon))
            (else
              (set `local.Socket` (`/Game/UsingData/Blueprint/Object/Non_SimulrationObject/Pair_Weapon/BP_PairWeapon.UnEquip Socket` _asbp_pair_weapon))))
          (switch `/Game/UsingData/Blueprint/Enum/Object/E_MeshType` (`/Game/UsingData/Blueprint/Object/Non_SimulrationObject/BP_Non_SimulationObject.Mesh Type` _asbp_pair_weapon)
            (:`NewEnumerator1`
              (`SceneComponent.K2_AttachToComponent` (`/Game/UsingData/Blueprint/Object/Non_SimulrationObject/BP_Non_SimulationObject.StaticMesh` _asbp_pair_weapon) (`self.Mesh`) (`local.Socket`) "KeepRelative" "KeepRelative" "KeepRelative" true))
            (:`NewEnumerator2`
              (`SceneComponent.K2_AttachToComponent` (`/Game/UsingData/Blueprint/Object/Non_SimulrationObject/BP_Non_SimulationObject.SkeletalMesh` _asbp_pair_weapon) (`self.Mesh`) (`local.Socket`) "KeepRelative" "KeepRelative" "KeepRelative" true))))))
    (:`then_1`
      (bind _asbp_weapon_object_2 (cast `/Game/UsingData/Blueprint/Object/SimulationObject/InteractionObject/MainWeaponObject/BP_WeaponObject` Actor)
        (:`then`
          (`/Game/UsingData/Blueprint/Object/SimulationObject/BP_SimulationObject.Set Visible` _asbp_weapon_object_2 _returnvalue))
        (:`CastFailed`
          (bind _asbp_pair_weapon_2 (cast `/Game/UsingData/Blueprint/Object/Non_SimulrationObject/Pair_Weapon/BP_PairWeapon` Actor))
          (`/Game/UsingData/Blueprint/Object/Non_SimulrationObject/BP_Non_SimulationObject.Set Visible` _asbp_pair_weapon_2 _returnvalue))))))

(fn `Can Action Skill`
  (params (`Skill Type` :type "/Game/UsingData/Blueprint/Enum/Weapon/E_SkillType Enum" :default "NewEnumerator0"))
  (returns (`Can Skill` :type Boolean))
  (if (`BlueprintMapLibrary.Map_Find` (`self.Skill Cool Time`) `Skill Type`)
    (switch `/Game/UsingData/Blueprint/Enum/Character/E_CharacterState` (`self.Character State`)
      (:`NewEnumerator0`
        (return true))
      (:`NewEnumerator4`
        _)
      (:`NewEnumerator23`
        _)
      (:`NewEnumerator26`
        _)
      (:`NewEnumerator27`
        _)
      (:`NewEnumerator24`
        _)
      (:`NewEnumerator21`
        _)
      (:`NewEnumerator22`
        _))
    (return false)
    (else
      (return false))))

(fn `Can Add Item`
  (params (`Item Name` :type "/Game/UsingData/Blueprint/Enum/Item/E_ItemName Enum" :default "NewEnumerator0"))
  (returns (`Can Add Item` :type Boolean))
  (bind _item_inventory (`self.Item Inventory`))
  (return (or (< (`BlueprintMapLibrary.Map_Length` _item_inventory) (`self.Max Item Inventory Num`)) (> (`BlueprintMapLibrary.Map_Find` _item_inventory (`local.Item Name`)) 0))))

(fn `Can Armming`
  (returns (`Can Armming` :type Boolean))
  (if (`self.Zoom Mode`)
    (return false)
    (else
      (switch `/Game/UsingData/Blueprint/Enum/Character/E_CharacterState` (`self.Character State`)
        (:`NewEnumerator0`
          _)
        (:`NewEnumerator4`
          (return false))
        (:`NewEnumerator23`
          (return false))
        (:`NewEnumerator26`
          (return false))
        (:`NewEnumerator27`
          (return false))
        (:`NewEnumerator24`
          (return false))
        (:`NewEnumerator28`
          _)
        (:`NewEnumerator30`
          (return false))
        (:`NewEnumerator21`
          (return false))
        (:`NewEnumerator29`
          (return false))
        (:`NewEnumerator22`
          (return false)))
      (return true))))

(fn `Can Attack`
  (returns (`Can Attack` :type Boolean))
  (switch `/Game/UsingData/Blueprint/Enum/Character/E_CharacterState` (`self.Character State`)
    (:`NewEnumerator0`
      (return true))
    (:`NewEnumerator4`
      _)
    (:`NewEnumerator23`
      _)
    (:`NewEnumerator26`
      _)
    (:`NewEnumerator27`
      _)
    (:`NewEnumerator24`
      _)
    (:`NewEnumerator28`
      _)
    (:`NewEnumerator30`
      _)
    (:`NewEnumerator21`
      _)
    (:`NewEnumerator29`
      _)
    (:`NewEnumerator22`
      _))
  (return false))

(fn `Can Dodge`
  (returns (`Can Dodge` :type Boolean))
  (switch `/Game/UsingData/Blueprint/Enum/Character/E_CharacterState` (`self.Character State`)
    (:`NewEnumerator0`
      _)
    (:`NewEnumerator4`
      _)
    (:`NewEnumerator23`
      _)
    (:`NewEnumerator26`
      _)
    (:`NewEnumerator27`
      _)
    (:`NewEnumerator24`
      (return false))
    (:`NewEnumerator28`
      (return false))
    (:`NewEnumerator30`
      _)
    (:`NewEnumerator21`
      _)
    (:`NewEnumerator29`
      _)
    (:`NewEnumerator22`
      (return false)))
  (return true))

(fn `Can Jump`
  (returns (`Can Jump` :type Boolean))
  (switch `/Game/UsingData/Blueprint/Enum/Character/E_CharacterState` (`self.Character State`)
    (:`NewEnumerator0`
      _)
    (:`NewEnumerator4`
      (return false))
    (:`NewEnumerator23`
      (return false))
    (:`NewEnumerator26`
      _)
    (:`NewEnumerator27`
      _)
    (:`NewEnumerator24`
      (return false))
    (:`NewEnumerator28`
      (return false))
    (:`NewEnumerator21`
      (return false))
    (:`NewEnumerator29`
      (return false))
    (:`NewEnumerator22`
      (return false)))
  (return true))

(fn `Can Move`
  (returns (`Can Move` :type Boolean))
  (switch `/Game/UsingData/Blueprint/Enum/Character/E_CharacterState` (`self.Character State`)
    (:`NewEnumerator0`
      (return true))
    (:`NewEnumerator4`
      _)
    (:`NewEnumerator23`
      _)
    (:`NewEnumerator26`
      _)
    (:`NewEnumerator27`
      _)
    (:`NewEnumerator24`
      _)
    (:`NewEnumerator28`
      _)
    (:`NewEnumerator30`
      _)
    (:`NewEnumerator21`
      _)
    (:`NewEnumerator29`
      _)
    (:`NewEnumerator22`
      _))
  (return false))

(fn `Can Pick Up Weapon`
  (params (`Weapon Name` :type "/Game/UsingData/Blueprint/Enum/Weapon/E_WeaponName Enum" :default "NewEnumerator0"))
  (returns (`Can Pick Up Weapon` :type Boolean))
  (if (< (`KismetArrayLibrary.Array_Length` (`self.Weapon Inventory`)) (`self.Max Weapon Inventory Num`))
    (for _array_element (`self.Weapon Inventory`)
      (bind _asbp_weapon_object (cast `/Game/UsingData/Blueprint/Object/SimulationObject/InteractionObject/MainWeaponObject/BP_WeaponObject` _array_element))
      (if (`|EnumEquality` (`/Game/UsingData/Blueprint/Object/SimulationObject/InteractionObject/MainWeaponObject/BP_WeaponObject.Weapon Name` _asbp_weapon_object) (`local.Weapon Name`))
        (return false)))
    (return true)
    (else
      (return false))))

(fn `Check Target`)

(fn `Is Character State`
  (params (`Character State` :type "/Game/UsingData/Blueprint/Enum/Character/E_CharacterState Enum" :default "NewEnumerator0"))
  (returns (Same :type Boolean))
  (return (`|EnumEquality` `Character State` (`self.Character State`))))

(fn `Set Die`
  (set `self.Character State` "NewEnumerator22"))

(fn `Update Hp Value`
  (locals (`Temp Hp Value Vector` :type "Array of /Game/UsingData/Blueprint/Structure/Character/S_Hp_Update_value Structure"))
  (for _array_element (`self.HP_Value_Vector`)
    (bind (_float _int _int2 _int3) (break `/Game/UsingData/Blueprint/Structure/Character/S_Hp_Update_value` _array_element))
    (if (== _int2 0)
      (set `self.Cur_Hp` (+ (`self.Cur_Hp`) _float))
      (bind _result (`/Engine/EditorBlueprintResources/StandardMacros.DecrementInt` _int)
        (:`  `
          (`KismetArrayLibrary.Array_Add` (`local.Temp Hp Value Vector`) (make `/Game/UsingData/Blueprint/Structure/Character/S_Hp_Update_value` _float _int _int3 _int3))))
      (else
        (`/Engine/EditorBlueprintResources/StandardMacros.DecrementInt` _int2
          (:`  `
            (`KismetArrayLibrary.Array_Add` (`local.Temp Hp Value Vector`) _array_element))))))
  (`|ExecutionSequence`
    (:`then_0`
      (if (> (`KismetArrayLibrary.Array_Length` (`local.Temp Hp Value Vector`)) 0)
        (set `self.HP_Value_Vector` (`local.Temp Hp Value Vector`))
        (else
          (`KismetSystemLibrary.K2_PauseTimerHandle` (`self.Hp_Update_Handle`))
          (`KismetArrayLibrary.Array_Clear` (`self.HP_Value_Vector`)))))
    (:`then_1`
      (bind _output_get (set `self.Cur_Hp` (`KismetMathLibrary.FClamp` (`self.Cur_Hp`) 0.0 (`self.Max_Hp`))))
      (if (== _output_get 0.0)
        (`self.Set Die`)))))

(fn `UserConstructionScript`)

(fn `Using Item`
  (params (`Item Name` :type "/Game/UsingData/Blueprint/Enum/Item/E_ItemName Enum" :default "NewEnumerator0") (`Item Num` :type Integer))
  (returns (Success :type Boolean))
  (if (> (`BlueprintMapLibrary.Map_Find` (`self.Item Inventory`) `Item Name`) `Item Num`)
    (`|ExecutionSequence`
      (:`then_0`
        (switch `/Game/UsingData/Blueprint/Enum/Item/E_ItemName` `Item Name`))
      (:`then_1`
        (return true)))))