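; BP_PlayerController turns player input into movement, camera look and action commands for the controlled pawn.
; Move axes apply yaw-relative movement when BP_Player allows it, and always store the axis values as dodge direction.
; Actions such as reload, zoom, crouch, jump, dodge, skills, weapon selection and speaker are forwarded as pawn messages.
; Button actions and certain full-value axis inputs call SetIsUserControl, which stops BP_Player's AI move-to-actor so manual control takes over.
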(event `InputAxis|MoveForward`
  (params (AxisValue :type "Float (single-precision)"))
  (bind (_returnvalue_roll _returnvalue_pitch _returnvalue_yaw) (`KismetMathLibrary.BreakRotator` (`self.GetControlRotation`)))
  (bind _asbp_player (cast `/Game/UsingData/Blueprint/Character/Player/BP_Player` (`self.K2_GetPawn`)))
  (bind _can_move (`/Game/UsingData/Blueprint/Character/BP_Character.Can Move` _asbp_player))
  (if _can_move
    (`Pawn.AddMovementInput` (`self.K2_GetPawn`) (`KismetMathLibrary.GetForwardVector` (`KismetMathLibrary.MakeRotator` 0.0 0.0 _returnvalue_yaw)) AxisValue false)
    (set `/Game/UsingData/Blueprint/Character/Player/BP_Player.Dodge Forward` AxisValue _asbp_player)
    (`self.Set Is User Control` (or (== AxisValue 1.0) (== AxisValue -1.0)))
    (else
      (set `/Game/UsingData/Blueprint/Character/Player/BP_Player.Dodge Forward` AxisValue _asbp_player))))

(event `InputAxis|MoveRight`
  (params (AxisValue :type "Float (single-precision)"))
  (bind (_returnvalue_roll _returnvalue_pitch _returnvalue_yaw) (`KismetMathLibrary.BreakRotator` (`self.GetControlRotation`)))
  (bind _asbp_player (cast `/Game/UsingData/Blueprint/Character/Player/BP_Player` (`self.K2_GetPawn`)))
  (bind _can_move (`/Game/UsingData/Blueprint/Character/BP_Character.Can Move` _asbp_player))
  (if _can_move
    (`Pawn.AddMovementInput` (`self.K2_GetPawn`) (`KismetMathLibrary.GetRightVector` (`KismetMathLibrary.MakeRotator` 0.0 0.0 _returnvalue_yaw)) AxisValue false)
    (set `/Game/UsingData/Blueprint/Character/Player/BP_Player.Dodge Right` AxisValue _asbp_player)
    (`self.Set Is User Control` (or (== AxisValue 1.0) (== AxisValue -1.0)))
    (else
      (set `/Game/UsingData/Blueprint/Character/Player/BP_Player.Dodge Right` AxisValue _asbp_player))))

(event `InputAxis|LookRight`
  (params (AxisValue :type "Float (single-precision)"))
  (`self.AddYawInput` AxisValue)
  (if (== AxisValue 1.0)
    (`self.Set Is User Control` true)))

(event `InputAxis|LookUp`
  (params (AxisValue :type "Float (single-precision)"))
  (`self.AddPitchInput` AxisValue)
  (if (== AxisValue -1.0)
    (`self.Set Is User Control` true)))

(event `InputAction|GunReload`
  (params (Key :type "Key Structure"))
  (:`Pressed`
    (message `/Game/UsingData/Blueprint/Interface/BPI_Character.Gun ReLoad` (`self.K2_GetPawn`))
    (`self.Set Is User Control` true)))

(event `InputAction|Action`
  (params (Key :type "Key Structure"))
  (:`Pressed`
    (message `/Game/UsingData/Blueprint/Interface/BPI_Character.Action` (`self.K2_GetPawn`))
    (`self.Set Is User Control` true)))

(event `InputAction|ActionDrop`
  (params (Key :type "Key Structure"))
  (:`Pressed`
    (message `/Game/UsingData/Blueprint/Interface/BPI_Character.Action Dropping` (`self.K2_GetPawn`))
    (`self.Set Is User Control` true)))

(event `InputAction|Zoom`
  (params (Key :type "Key Structure"))
  (bind _returnvalue (`self.K2_GetPawn`))
  (:`Pressed`
    (message `/Game/UsingData/Blueprint/Interface/BPI_Character.Zoom Camera In` _returnvalue)
    (`self.Set Is User Control` true :!label _label))
  (:`Released`
    (message `/Game/UsingData/Blueprint/Interface/BPI_Character.Zoom Camera Out` _returnvalue)
    (goto _label)))

(event `InputAction|EquipOrUnEuip`
  (params (Key :type "Key Structure"))
  (:`Pressed`
    (message `/Game/UsingData/Blueprint/Interface/BPI_Character.Equp Or UnEquip` (`self.K2_GetPawn`))
    (`self.Set Is User Control` true)))

(event `InputAction|Crouch`
  (params (Key :type "Key Structure"))
  (bind _returnvalue (`self.K2_GetPawn`))
  (:`Pressed`
    (message `/Game/UsingData/Blueprint/Interface/BPI_Character.Character Crouch` _returnvalue true)
    (`self.Set Is User Control` true :!label _label_2))
  (:`Released`
    (message `/Game/UsingData/Blueprint/Interface/BPI_Character.Character Crouch` _returnvalue false)
    (goto _label_2)))

(event `InputAction|Jump`
  (params (Key :type "Key Structure"))
  (bind _returnvalue (`self.K2_GetPawn`))
  (:`Pressed`
    (message `/Game/UsingData/Blueprint/Interface/BPI_Character.Character Jump` _returnvalue true)
    (`self.Set Is User Control` true :!label _label_3))
  (:`Released`
    (message `/Game/UsingData/Blueprint/Interface/BPI_Character.Character Jump` _returnvalue false)
    (goto _label_3)))

(event `InputAction|Dodge`
  (params (Key :type "Key Structure"))
  (:`Pressed`
    (message `/Game/UsingData/Blueprint/Interface/BPI_Character.ActionDodge` (`self.K2_GetPawn`))
    (`self.Set Is User Control` true)))

(event `InputAction|Skill_1`
  (params (Key :type "Key Structure"))
  (:`Pressed`
    (message `/Game/UsingData/Blueprint/Interface/BPI_Character.Skill` (`self.K2_GetPawn`) "NewEnumerator0")
    (`self.Set Is User Control` true :!label _label_4)))

(event `InputAction|Weapon_1`
  (params (Key :type "Key Structure"))
  (:`Pressed`
    (message `/Game/UsingData/Blueprint/Interface/BPI_Character.Weapon_Select` (`self.K2_GetPawn`) 0)
    (`self.Set Is User Control` true :!label _label_5)))

(event `InputAction|Weapon_2`
  (params (Key :type "Key Structure"))
  (:`Pressed`
    (message `/Game/UsingData/Blueprint/Interface/BPI_Character.Weapon_Select` (`self.K2_GetPawn`) 1)
    (goto _label_5)))

(event `InputAction|Skill_2`
  (params (Key :type "Key Structure"))
  (:`Pressed`
    (message `/Game/UsingData/Blueprint/Interface/BPI_Character.Skill` (`self.K2_GetPawn`) "NewEnumerator1")
    (goto _label_4)))

(event `InputAction|Weapon_3`
  (params (Key :type "Key Structure"))
  (:`Pressed`
    (message `/Game/UsingData/Blueprint/Interface/BPI_Character.Weapon_Select` (`self.K2_GetPawn`) 2)
    (goto _label_5)))

(event `InputAction|Skill_3`
  (params (Key :type "Key Structure"))
  (:`Pressed`
    (message `/Game/UsingData/Blueprint/Interface/BPI_Character.Skill` (`self.K2_GetPawn`) "NewEnumerator2")
    (goto _label_4)))

(event `InputAction|Weapon_4`
  (params (Key :type "Key Structure"))
  (:`Pressed`
    (message `/Game/UsingData/Blueprint/Interface/BPI_Character.Weapon_Select` (`self.K2_GetPawn`) 3)
    (goto _label_5)))

(event `InputAction|Skill_4`
  (params (Key :type "Key Structure"))
  (:`Pressed`
    (message `/Game/UsingData/Blueprint/Interface/BPI_Character.Skill` (`self.K2_GetPawn`) "NewEnumerator3")
    (goto _label_4)))

(event `InputAxis|speaker`
  (params (AxisValue :type "Float (single-precision)"))
  (if (== AxisValue 1.0)
    (message `/Game/UsingData/Blueprint/Interface/BPI_Character.Speaker` (`self.K2_GetPawn`))
    (`self.Set Is User Control` true)))

(fn `Set Is User Control`
  (params (`is User Control` :type Boolean))
  (if `is User Control`
    (bind _asbp_player (cast `/Game/UsingData/Blueprint/Character/Player/BP_Player` (`self.K2_GetPawn`)))
    (`/Game/UsingData/Blueprint/Character/Player/BP_Player.Stop AI Move To Actor` _asbp_player)))

(fn `UserConstructionScript`)