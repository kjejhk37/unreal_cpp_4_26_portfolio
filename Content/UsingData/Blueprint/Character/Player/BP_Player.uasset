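; Player character Blueprint that handles dodging and item pickup on top of a parent character class.
; Dodge cancels active weapon effects when attacking, stops montages, sets the Dodge state and plays a montage that resets state on completion.
; A separate event turns the mesh toward camera-relative dodge input using dot and cross products.
; BeginPlay spawns a gun spawner targeting the player; successful interaction overlaps stop AI movement and add to inventory.
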(event `Set Dodge Direction`
  (bind (_returnvalue_roll _returnvalue_pitch _returnvalue_yaw) (`KismetMathLibrary.BreakRotator` (`self.GetControlRotation`)))
  (bind _mesh (`self.Mesh`))
  (bind _returnvalue (`SceneComponent.GetRightVector` (`self.Mesh`)))
  (bind _returnvalue_2 (`KismetMathLibrary.Normal` (+ (* (`KismetMathLibrary.GetForwardVector` (`KismetMathLibrary.MakeRotator` 0.0 0.0 _returnvalue_yaw)) (`self.Dodge Forward`)) (* (`KismetMathLibrary.GetRightVector` (`KismetMathLibrary.MakeRotator` 0.0 0.0 _returnvalue_yaw)) (`self.Dodge Right`)))))
  (bind (_returnvalue_x _returnvalue_y _returnvalue_z) (`KismetMathLibrary.BreakVector` (`KismetMathLibrary.Cross_VectorVector` _returnvalue _returnvalue_2)))
  (bind _returnvalue_3 (`KismetMathLibrary.DegAcos` (`KismetMathLibrary.Dot_VectorVector` _returnvalue _returnvalue_2)))
  (if (> _returnvalue_z 0.0)
    (`SceneComponent.K2_AddRelativeRotation` _mesh (`KismetMathLibrary.MakeRotator` 0.0 0.0 _returnvalue_3) false false)
    (else
      (`SceneComponent.K2_AddRelativeRotation` _mesh (`KismetMathLibrary.MakeRotator` 0.0 0.0 (* _returnvalue_3 -1.0)) false false))))

(event `self.ReceiveBeginPlay`
  (`parent.ReceiveBeginPlay`)
  (bind _returnvalue (`|SpawnActorFromClass` "/Game/UsingData/Blueprint/Skill/Spawn_Skill/BP_Spawn_Gun.BP_Spawn_Gun_C" (`KismetMathLibrary.MakeTransform` (0.0 0.0 0.0)) "Undefined" "OverrideRootScale" null null))
  (`/Game/UsingData/Blueprint/Skill/Spawn_Skill/BP_Spawn.Set Spawn` _returnvalue (-100.0 0.0 50.0) self)
  (`/Game/UsingData/Blueprint/Skill/BP_Skill.Play` _returnvalue true))

(event `self.Interaction Collision.OnComponentBeginOverlap`
  (params (OverlappedComponent :type "PrimitiveComponent Object Reference") (OtherActor :type "Actor Object Reference") (OtherComp :type "PrimitiveComponent Object Reference") (OtherBodyIndex :type Integer) (bFromSweep :type Boolean) (SweepResult :type "HitResult Structure (by ref)"))
  (bind _asbp_interaction_object (cast `/Game/UsingData/Blueprint/Object/SimulationObject/InteractionObject/BP_InteractionObject` OtherActor))
  (bind (_interaction_success _result_actor) (message `/Game/UsingData/Blueprint/Interface/BPI_Interaction.Interaction` _asbp_interaction_object self))
  (if _interaction_success
    (`self.Stop AI Move To Actor`)
    (`self.Add Inventory` _interaction_success _result_actor)))

(event `self.ActionDodge`
  (bind _returnvalue (`SkeletalMeshComponent.GetAnimInstance` (`self.Mesh`)))
  (bind _can_dodge (`self.Can Dodge`))
  (if _can_dodge
    (`self.Set Before Dodge`)
    (`/Engine/EditorBlueprintResources/StandardMacros.IsValid` _returnvalue
      (:`Is Valid`
        (`AnimInstance.Montage_Stop` _returnvalue 0.0 null))
      (:`Is Not Valid`
        _))
    (set `self.Character State` "NewEnumerator24")
    (`self.Main Weapon`
      (:`then`
        _)
      (:`else`
        _))
    (bind _notifyname (`|PlayMontage` (`self.Mesh`) "/Game/CBP_Data/BP/Character/Player/PlayerAnimation/Montage/Dodge/Player_Dodge.Player_Dodge" 1.5)
      (:`OnCompleted`
        (`self.ReSetState`))
      (:`OnNotifyBegin`
        (switch `name` _notifyname))
      (:`OnNotifyEnd`
        (switch `name` _notifyname)))))

(event `self.ReSetState`
  (`parent.ReSetState`))

(event `self.Action`
  (`parent.Action`)
  (`self.Main Weapon`
    (:`then`)
    (:`else`)))

(fn `Set Before Dodge`
  (bind _main_weapon (`self.Main Weapon`))
  (bind _pair_weapon (`self.Pair Weapon`))
  (switch `/Game/UsingData/Blueprint/Enum/Character/E_CharacterState` (`self.Character State`)
    (:`NewEnumerator4`
      (message `/Game/UsingData/Blueprint/Interface/BPI_Weapon.Deactivate` _main_weapon true)
      (message `/Game/UsingData/Blueprint/Interface/BPI_Trail_Particle_Weapon.Particle_DeActivate` _main_weapon)
      (message `/Game/UsingData/Blueprint/Interface/BPI_Weapon.Deactivate` _pair_weapon true)
      (message `/Game/UsingData/Blueprint/Interface/BPI_Trail_Particle_Weapon.Particle_DeActivate` _pair_weapon))))

(fn `Stop AI Move To Actor`
  (`Controller.StopMovement` (`self.GetController`)))

(fn `UserConstructionScript`
  (`parent.UserConstructionScript`))