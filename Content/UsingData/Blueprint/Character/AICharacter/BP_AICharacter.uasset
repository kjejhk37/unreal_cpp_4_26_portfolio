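; BP_AICharacter is an AI-controlled character that detects hostile BP_Characters, judged by comparing camps, through its AIPerception component.
; Perception updates add or remove hostiles in a Targets list based on sight.
; Hearing records the noise position and raises IsHearing only while that list is empty.
; SearchNearTarget switches CurTarget to the first listed target closer than the current one, or clears it when none remain.
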(event `self.AIPerception.OnTargetPerceptionUpdated`
  (params (Actor :type "Actor Object Reference") (Stimulus :type "AIStimulus Structure"))
  (bind _asbp_character (cast `/Game/UsingData/Blueprint/Character/BP_Character` Actor))
  (if (`/Game/UsingData/Blueprint/Define/BPF_Function.Get hostile` (`self.Camp`) (`/Game/UsingData/Blueprint/Character/BP_Character.Camp` _asbp_character))
    (`self.Set Sight` Actor)
    (`self.Set Hearing` Actor)))

(fn `Search Near Target`
  (bind _targets (`self.Targets`))
  (if (== (`KismetArrayLibrary.Array_Length` _targets) 0)
    (set `self.Cur Target` null)
    (else
      (for _array_element _targets
        (if (!= _array_element (`self.Cur Target`))
          (if (< (`KismetMathLibrary.VSize` (- (`self.K2_GetActorLocation` _array_element) (`self.K2_GetActorLocation`))) (`KismetMathLibrary.VSize` (- (`self.K2_GetActorLocation` (`self.Cur Target`)) (`self.K2_GetActorLocation`))))
            (set `self.Cur Target` _array_element)
            (return)))))))

(fn `Set Hearing`
  (params (Actor :type "Actor Object Reference"))
  (if (> (`KismetArrayLibrary.Array_Length` (`self.Targets`)) 0)
    _
    (elif (`KismetArrayLibrary.Array_Contains` (`AIPerceptionComponent.GetCurrentlyPerceivedActors` (`self.AIPerception`) "/Script/AIModule.AISense_Hearing") Actor)
      (set `self.Hearing Position` (`self.K2_GetActorLocation` Actor))
      (set `self.is Hearing` true))))

(fn `Set Sight`
  (params (Actor :type "Actor Object Reference"))
  (bind _targets (`self.Targets`))
  (if (`KismetArrayLibrary.Array_Contains` (`AIPerceptionComponent.GetCurrentlyPerceivedActors` (`self.AIPerception`) "/Script/AIModule.AISense_Sight") Actor)
    (`KismetArrayLibrary.Array_Add` _targets Actor)
    (else
      (`KismetArrayLibrary.Array_RemoveItem` _targets Actor))))

(fn `UserConstructionScript`
  (`parent.UserConstructionScript`))