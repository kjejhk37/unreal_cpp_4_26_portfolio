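; BP_shielddestroy is a magic-effect Blueprint for a shield-destroy visual with configurable color and brightness.
; On BeginPlay it creates dynamic material instances for eight element slots, applying the shield settings to the first two and the circle settings to the other six.
; Tick runs a short Delay, then calls Activate without reset, so activation repeats periodically rather than firing once.
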(event `self.ReceiveBeginPlay`
  (bind _color_shield (`self.color_shield`))
  (bind _color_circle (`self.color_circle`))
  (bind _brightness_shield (`self.brightness_shield`))
  (bind _brightness_circle (`self.brightness_circle`))
  (bind _returnvalue (`PrimitiveComponent.CreateDynamicMaterialInstance` 0 null))
  (`MaterialInstanceDynamic.SetScalarParameterValue` _returnvalue "br" _brightness_shield)
  (`MaterialInstanceDynamic.SetVectorParameterValue` _returnvalue "color" _color_shield)
  (bind _returnvalue_2 (`PrimitiveComponent.CreateDynamicMaterialInstance` 1 null))
  (`MaterialInstanceDynamic.SetScalarParameterValue` _returnvalue_2 "br" _brightness_shield)
  (`MaterialInstanceDynamic.SetVectorParameterValue` _returnvalue_2 "color" _color_shield)
  (bind _returnvalue_3 (`PrimitiveComponent.CreateDynamicMaterialInstance` 2 null))
  (`MaterialInstanceDynamic.SetScalarParameterValue` _returnvalue_3 "br" _brightness_circle)
  (`MaterialInstanceDynamic.SetVectorParameterValue` _returnvalue_3 "color" _color_circle)
  (bind _returnvalue_4 (`PrimitiveComponent.CreateDynamicMaterialInstance` 3 null))
  (`MaterialInstanceDynamic.SetScalarParameterValue` _returnvalue_4 "br" _brightness_circle)
  (`MaterialInstanceDynamic.SetVectorParameterValue` _returnvalue_4 "color" _color_circle)
  (bind _returnvalue_5 (`PrimitiveComponent.CreateDynamicMaterialInstance` 4 null))
  (`MaterialInstanceDynamic.SetScalarParameterValue` _returnvalue_5 "br" _brightness_circle)
  (`MaterialInstanceDynamic.SetVectorParameterValue` _returnvalue_5 "color" _color_circle)
  (bind _returnvalue_6 (`PrimitiveComponent.CreateDynamicMaterialInstance` 5 null))
  (`MaterialInstanceDynamic.SetScalarParameterValue` _returnvalue_6 "br" _brightness_circle)
  (`MaterialInstanceDynamic.SetVectorParameterValue` _returnvalue_6 "color" _color_circle)
  (bind _returnvalue_7 (`PrimitiveComponent.CreateDynamicMaterialInstance` 6 null))
  (`MaterialInstanceDynamic.SetScalarParameterValue` _returnvalue_7 "br" _brightness_circle)
  (`MaterialInstanceDynamic.SetVectorParameterValue` _returnvalue_7 "color" _color_circle)
  (bind _returnvalue_8 (`PrimitiveComponent.CreateDynamicMaterialInstance` 7 null))
  (`MaterialInstanceDynamic.SetScalarParameterValue` _returnvalue_8 "br" _brightness_circle)
  (`MaterialInstanceDynamic.SetVectorParameterValue` _returnvalue_8 "color" _color_circle))

(event `self.ReceiveTick`
  (params (DeltaSeconds :type "Float (single-precision)"))
  (`KismetSystemLibrary.Delay` 0.2)
  (`ActorComponent.Activate` false))

(fn `UserConstructionScript`)