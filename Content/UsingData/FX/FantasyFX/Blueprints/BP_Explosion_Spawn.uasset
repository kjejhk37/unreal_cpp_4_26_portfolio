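; Fantasy FX spawner actor that fires repeating five-shot volleys of BP_Explosion_Projectile while IsActive is set.
; Tick passes through a DoOnce into a delayed Sequence that staggers the shots, then resets and loops after a pause.
; Each shot spawns at Arrow's location with one of five arrow rotations and a random speed above ProjectileSpeedMin.
; A shared spark component is turned to each shot's direction and briefly activated.
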(event `self.ReceiveTick`
  (params (DeltaSeconds :type "Float (single-precision)"))
  (bind _p_poisonball_spawn_sparks (`self.P_PoisonBall_Spawn_Sparks`))
  (bind _p_poisonball_spawn_sparks_2 (`self.P_PoisonBall_Spawn_Sparks`))
  (bind _projectilespeedmin (`self.ProjectileSpeedMin`))
  (bind _projectilespeedmin_2 (`self.ProjectileSpeedMin`))
  (bind _projectilespeedmin_3 (`self.ProjectileSpeedMin`))
  (bind _projectilespeedmin_4 (`self.ProjectileSpeedMin`))
  (bind _projectilespeedmin_5 (`self.ProjectileSpeedMin`))
  (bind _p_poisonball_spawn_sparks_3 (`self.P_PoisonBall_Spawn_Sparks`))
  (bind _p_poisonball_spawn_sparks_4 (`self.P_PoisonBall_Spawn_Sparks`))
  (bind _p_poisonball_spawn_sparks_5 (`self.P_PoisonBall_Spawn_Sparks`))
  (bind _returnvalue (`SceneComponent.K2_GetComponentRotation` (`self.Arrow2`)))
  (bind _returnvalue_2 (`SceneComponent.K2_GetComponentRotation` (`self.Arrow3`)))
  (bind _returnvalue_3 (`SceneComponent.K2_GetComponentRotation` (`self.Arrow4`)))
  (bind _returnvalue_4 (`SceneComponent.K2_GetComponentRotation` (`self.Arrow`)))
  (bind _returnvalue_5 (`SceneComponent.K2_GetComponentRotation` (`self.Arrow1`)))
  (if (`self.IsActive`) :!label _label
    (`/Engine/EditorBlueprintResources/StandardMacros.DoOnce` false :!label _label_2
      (:`Completed`
        (`KismetSystemLibrary.Delay` 1.0)
        (`|ExecutionSequence`
          (:`then_0`
            (`SceneComponent.K2_SetWorldRotation` _p_poisonball_spawn_sparks_3 _returnvalue_3 false false)
            (`ActorComponent.SetActive` _p_poisonball_spawn_sparks_3 true false)
            (`|SpawnActorFromClass` "/Game/UsingData/FX/FantasyFX/Blueprints/BP_Explosion_Projectile.BP_Explosion_Projectile_C" (`KismetMathLibrary.MakeTransform` (`SceneComponent.K2_GetComponentLocation` (`self.Arrow`)) _returnvalue_3) "AlwaysSpawn" "OverrideRootScale" null (`KismetMathLibrary.Conv_IntToDouble` (`KismetMathLibrary.RandomIntegerInRange` _projectilespeedmin (+ _projectilespeedmin 500))) null)
            (`KismetSystemLibrary.Delay` 0.1)
            (`ActorComponent.SetActive` (`self.P_PoisonBall_Spawn_Sparks`) false false))
          (:`then_1`
            (`KismetSystemLibrary.Delay` 0.1)
            (`SceneComponent.K2_SetWorldRotation` _p_poisonball_spawn_sparks_4 _returnvalue_4 false false)
            (`ActorComponent.SetActive` _p_poisonball_spawn_sparks_4 true false)
            (`|SpawnActorFromClass` "/Game/UsingData/FX/FantasyFX/Blueprints/BP_Explosion_Projectile.BP_Explosion_Projectile_C" (`KismetMathLibrary.MakeTransform` (`SceneComponent.K2_GetComponentLocation` (`self.Arrow`)) _returnvalue_4) "AlwaysSpawn" "OverrideRootScale" null (`KismetMathLibrary.Conv_IntToDouble` (`KismetMathLibrary.RandomIntegerInRange` _projectilespeedmin_5 (+ _projectilespeedmin_5 500))) null)
            (`KismetSystemLibrary.Delay` 0.1)
            (`ActorComponent.SetActive` (`self.P_PoisonBall_Spawn_Sparks`) false false))
          (:`then_2`
            (`KismetSystemLibrary.Delay` 0.2)
            (`SceneComponent.K2_SetWorldRotation` _p_poisonball_spawn_sparks_5 _returnvalue_5 false false)
            (`ActorComponent.SetActive` _p_poisonball_spawn_sparks_5 true false)
            (`|SpawnActorFromClass` "/Game/UsingData/FX/FantasyFX/Blueprints/BP_Explosion_Projectile.BP_Explosion_Projectile_C" (`KismetMathLibrary.MakeTransform` (`SceneComponent.K2_GetComponentLocation` (`self.Arrow`)) _returnvalue_5) "AlwaysSpawn" "OverrideRootScale" null (`KismetMathLibrary.Conv_IntToDouble` (`KismetMathLibrary.RandomIntegerInRange` _projectilespeedmin_4 (+ _projectilespeedmin_4 500))) null)
            (`KismetSystemLibrary.Delay` 0.1)
            (`ActorComponent.SetActive` (`self.P_PoisonBall_Spawn_Sparks`) false false))
          (:`then_3`
            (`KismetSystemLibrary.Delay` 0.3)
            (`SceneComponent.K2_SetWorldRotation` _p_poisonball_spawn_sparks _returnvalue false false)
            (`ActorComponent.SetActive` _p_poisonball_spawn_sparks true false)
            (`|SpawnActorFromClass` "/Game/UsingData/FX/FantasyFX/Blueprints/BP_Explosion_Projectile.BP_Explosion_Projectile_C" (`KismetMathLibrary.MakeTransform` (`SceneComponent.K2_GetComponentLocation` (`self.Arrow`)) _returnvalue) "AlwaysSpawn" "OverrideRootScale" null (`KismetMathLibrary.Conv_IntToDouble` (`KismetMathLibrary.RandomIntegerInRange` _projectilespeedmin_3 (+ _projectilespeedmin_3 500))) null)
            (`KismetSystemLibrary.Delay` 0.1)
            (`ActorComponent.SetActive` (`self.P_PoisonBall_Spawn_Sparks`) false false))
          (:`then_4`
            (`KismetSystemLibrary.Delay` 0.4)
            (`SceneComponent.K2_SetWorldRotation` _p_poisonball_spawn_sparks_2 _returnvalue_2 false false)
            (`ActorComponent.SetActive` _p_poisonball_spawn_sparks_2 true false)
            (`|SpawnActorFromClass` "/Game/UsingData/FX/FantasyFX/Blueprints/BP_Explosion_Projectile.BP_Explosion_Projectile_C" (`KismetMathLibrary.MakeTransform` (`SceneComponent.K2_GetComponentLocation` (`self.Arrow`)) _returnvalue_2) "AlwaysSpawn" "OverrideRootScale" null (`KismetMathLibrary.Conv_IntToDouble` (`KismetMathLibrary.RandomIntegerInRange` _projectilespeedmin_2 (+ _projectilespeedmin_2 500))) null)
            (`KismetSystemLibrary.Delay` 0.1)
            (`ActorComponent.SetActive` (`self.P_PoisonBall_Spawn_Sparks`) false false)
            (`KismetSystemLibrary.Delay` 3.0)
            (`|ExecutionSequence`
              (:`then_0`
                (goto _label_2 :!via `Reset`))
              (:`then_1`
                (goto _label)))))))
    (else
      (goto _label_2 :!via `Reset`))))

(fn `UserConstructionScript`)