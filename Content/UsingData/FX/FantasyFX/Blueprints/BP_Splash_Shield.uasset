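; BP_Splash_Shield is a visual effect actor that plays a timed splash shield animation on a sphere mesh after a one-second delay.
; Timelines animate the dynamic material's Percent and staggered EmissiveLerp, and the particle system activates when the Percent animation ends.
; When the emissive lerp ends, the sphere switches to M_Splash_Shield2 for a final emissive timeline.
; Tick billboards the Scene component by aligning it to the direction from the player camera.
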(event `self.ReceiveBeginPlay`
  (bind _sphere (`self.Sphere`))
  (`KismetSystemLibrary.Delay` 1.0)
  (bind _returnvalue (`PrimitiveComponent.CreateDynamicMaterialInstance` _sphere 0 (`PrimitiveComponent.GetMaterial` _sphere 0) "None"))
  (`|ExecutionSequence`
    (:`then_0`
      (bind (_direction _newtrack_0) (`Timeline|ScaleTexture` :!via `PlayFromStart`)
        (:`Update`
          (`MaterialInstanceDynamic.SetScalarParameterValue` _returnvalue "Percent" _newtrack_0))
        (:`Finished`
          (`ActorComponent.SetActive` (`self.ParticleSystem`) true false))))
    (:`then_1`
      (`KismetSystemLibrary.Delay` 0.45)
      (bind (_direction_2 _newtrack_0_2) (`Timeline|EmissiveLerp` :!via `PlayFromStart`)
        (:`Update`
          (`MaterialInstanceDynamic.SetScalarParameterValue` _returnvalue "EmissiveLerp" _newtrack_0_2))
        (:`Finished`
          (bind _returnvalue_2 (`PrimitiveComponent.CreateDynamicMaterialInstance` (`self.Sphere`) 0 "/Game/UsingData/FX/FantasyFX/Materials/Splash/M_Splash_Shield2.M_Splash_Shield2" "None"))
          (`MaterialInstanceDynamic.SetScalarParameterValue` _returnvalue_2 "Percent" 0.0)
          (bind (_direction_3 _newtrack_0_3) (`Timeline|Timeline_0` :!via `PlayFromStart`)
            (:`Update`
              (`MaterialInstanceDynamic.SetScalarParameterValue` _returnvalue_2 "EmissiveLerp" _newtrack_0_3))))))))

(event `self.ReceiveTick`
  (params (DeltaSeconds :type "Float (single-precision)"))
  (bind _scene (`self.Scene`))
  (`SceneComponent.K2_SetWorldRotation` _scene (`KismetMathLibrary.FindLookAtRotation` (`PlayerCameraManager.GetCameraLocation` (`GameplayStatics.GetPlayerCameraManager` 0)) (`SceneComponent.K2_GetComponentLocation` _scene)) false false))

(fn `UserConstructionScript`)